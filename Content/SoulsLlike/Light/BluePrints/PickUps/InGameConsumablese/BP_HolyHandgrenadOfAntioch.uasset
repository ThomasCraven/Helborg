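; Holy Hand Grenade of Antioch, a projectile consumable with a looping fuse sound that explodes and damages enemies and players.
; Each bounce sets a one-second timer, while the first also enables sphere physics and starts a timeline driving the dynamic material's Alpha.
; Expload sphere-traces the blast radius and sends damage messages to actors implementing the enemy or player interface.
; Destory then plays force feedback, sound and two Niagara effects before destroying the actor.
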(event OnProjectileBounce(ProjectileMovement)
  (params (ImpactResult :type Hit%20Result%20Structure%20%28by%20ref%29) (ImpactVelocity :type Vector%20%28by%20ref%29 :default "0, 0, 0"))
  (bind _returnvalue (Utilities|Time|SetTimerbyEvent (EventDispatchers|CreateEvent :!event Expload) 1.0))
  (Variables|Default|SetExploadHandle _returnvalue)
  (Utilities|FlowControl|DoOnce false
    (:Completed
      (Physics|SetSimulatePhysics (Variables|Default|GetSphere) true)
      (bind _alpha (Timeline|TickTickTimer Play)
        (:Update
          (Rendering|Material|SetScalarParameterValue (Variables|Default|GetBoomMaterial) "Alpha" _alpha :!class /Script/Engine.MaterialInstanceDynamic))))))

(event EventBeginPlay
  (bind _returnvalue (Rendering|Material|CreateDynamicMaterialInstance (Variables|Default|GetStaticMesh) 0 "/Game/SoulsLlike/Heavy/Matarials/Game/M_Dungeon_01_Inst.M_Dungeon_01_Inst" "None" :!class /Script/Engine.PrimitiveComponent))
  (Variables|Default|SetBoomMaterial _returnvalue)
  (bind _returnvalue_2 (Audio|SpawnSoundAttached "/Game/SoulsLlike/Light/Sound/Effects/SW_Dynamite_Fuse_Loop_001.SW_Dynamite_Fuse_Loop_001" (Variables|Default|GetArrow) "None" "0, 0, 0" "0, 0, 0" "KeepRelativeOffset" false 1.0 1.0 0.0 0 0))
  (Variables|Default|SetFuseSound _returnvalue_2))

(fn ConstructionScript
  (|CallParentFunction))

(fn Expload
  (bind _returnvalue (Transformation|GetActorLocation))
  (bind _outhits (Collision|MultiSphereTraceByChannel _returnvalue _returnvalue 4e+02 "TraceTypeQuery1" true 0 "None"))
  (for _array_element _outhits
    (if (CallFunction|CanHit? (.HitActor (Collision|BreakHitResult _array_element)))
      (Class|BPIEnemy|Damage(Message) (.HitActor (Collision|BreakHitResult _array_element)) (Variables|Default|GetDamage%20Enemy))
      (Class|BPIPlayer|AttackPlayer(Message) (.HitActor (Collision|BreakHitResult _array_element)) (Variables|Default|GetDamage%20Player))))
  (CallFunction|Destory))

(fn CanHit?
  (params (Actor :type Object%20Object%20Reference))
  (if (or (Utilities|DoesObjectImplementInterface Actor "/Game/SoulsLlike/Light/BluePrints/Interfaces/BPI_Enemy.BPI_Enemy_C") (Utilities|DoesObjectImplementInterface Actor "/Game/SoulsLlike/Light/BluePrints/Interfaces/BPI_Player.BPI_Player_C"))
    (return true)
    (else
      (return false))))

(fn Destory
  (bind _arrow (Variables|Default|GetArrow))
  (bind _returnvalue (Transformation|GetSocketLocation _arrow "None"))
  (ForceFeedback|SpawnForceFeedbackatLocation "/Game/SoulsLlike/Light/Inputs/Feedback/FF_MegaHigh.FF_MegaHigh" (Transformation|GetSocketLocation (Variables|Default|GetArrow) "None") "0, 0, 0" false 1.0 0.0 0)
  (Audio|Components|Audio|Stop (Variables|Default|GetFuseSound))
  (Audio|PlaySoundatLocation "/Game/SoulsLlike/Light/Sound/Effects/SW_Frag_Grenade_003.SW_Frag_Grenade_003" _returnvalue "0, 0, 0" 1.0 1.0 0.0 0 0 0 0)
  (Niagara|SpawnSystematLocation "/Game/SoulsLlike/Heavy/Systems/NS_BoomGold.NS_BoomGold" _returnvalue)
  (Niagara|SpawnSystematLocation "/Game/SoulsLlike/Heavy/Systems/NS_Boom.NS_Boom" (Transformation|GetSocketLocation (Variables|Default|GetArrow) "None"))
  (Utilities|Time|ClearandInvalidateTimerbyHandle (Variables|Default|GetExploadHandle))
  (Actor|DestroyActor))