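; BP_PickUpItem is a world item pickup that offers an item from a data asset, with a settable amount, to the player.
; Box overlap or OpenPickup shows the item popup through BPCPopUpUI; leaving the box dismisses it.
; Interact checks the player's popup asset matches, passes item and amount via ItemPickUpMessage, then on success hides the pickup and disables collision.
; PickedUp separately plays a sound and destroys the actor.
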(event OnComponentBeginOverlap(Box)
  (params (OverlappedComponent :type Primitive%20Component%20Object%20Reference) (OtherActor :type Actor%20Object%20Reference) (OtherComp :type Primitive%20Component%20Object%20Reference) (OtherBodyIndex :type Integer) (bFromSweep :type Boolean) (SweepResult :type Hit%20Result%20Structure%20%28by%20ref%29))
  (bind _itemdata (Variables|Default|GetItemData))
  (bind _iteminfo (Variables|/Game/SoulsLlike/Light/DataAssets/BPD_ItemData.BPD_ItemData_C|GetItemInfo _itemdata))
  (bind (_icon _name) (Utilities|Struct|BreakStruct_ItemHeader _iteminfo))
  (Variables|Default|SetOther%20Comp OtherComp)
  (Variables|Default|SetPlayer OtherActor)
  (Default|PopUp (Variables|Default|GetBPC_PopUpUI) _name (Variables|Default|GetPlayer) _icon "NewEnumerator1" (Variables|Default|GetItemAmount) (Variables|Default|GetOther%20Comp) _itemdata self))

(event OnComponentEndOverlap(Box)
  (params (OverlappedComponent :type Primitive%20Component%20Object%20Reference) (OtherActor :type Actor%20Object%20Reference) (OtherComp :type Primitive%20Component%20Object%20Reference) (OtherBodyIndex :type Integer))
  (Default|LeavePopUp (Variables|Default|GetBPC_PopUpUI) OtherActor OtherComp))

(event EventAddAmount
  (params (AmountToAdd :type Integer))
  (Variables|Default|SetItemAmount AmountToAdd))

(event EventOpenPickup
  (params (player :type BP%20Base%20Souls%20Chap%20Object%20Reference) (Component :type Primitive%20Component%20Object%20Reference))
  (bind _itemdata (Variables|Default|GetItemData))
  (bind _iteminfo (Variables|/Game/SoulsLlike/Light/DataAssets/BPD_ItemData.BPD_ItemData_C|GetItemInfo _itemdata))
  (bind (_icon _name) (Utilities|Struct|BreakStruct_ItemHeader _iteminfo))
  (Variables|Default|SetOther%20Comp Component)
  (Variables|Default|SetPlayer player)
  (Default|PopUp (Variables|Default|GetBPC_PopUpUI) _name (Variables|Default|GetPlayer) _icon "NewEnumerator1" (Variables|Default|GetItemAmount) (Variables|Default|GetOther%20Comp) _itemdata self))

(fn ConstructionScript)

(fn PickedUp
  (Audio|PlaySound2D "/Game/SoulsLlike/Light/Sound/Effects/SW_Stone_Ward_001.SW_Stone_Ward_001" 1.0 1.0 0.0 0 0)
  (Actor|DestroyActor))

(fn Interact
  (params (HasIntracted? :type Boolean) (Player :type BP%20Base%20Souls%20Chap%20Object%20Reference))
  (if (== (Variables|/Game/SoulsLlike/Light/BluePrints/Player/BP_BaseSoulsChap.BP_BaseSoulsChap_C|GetData%20Asset%20Popup Player) (Variables|Default|GetItemData))
    (bind _haassent (Class|BPIPlayer|ItemPickUp(Message) Player (Variables|Default|GetItemAmount) (Variables|Default|GetItemData)))
    (if _haassent
      (Default|LeavePopUp (Variables|Default|GetBPC_PopUpUI) Player (Variables|Default|GetOther%20Comp))
      (Rendering|SetVisibility (Variables|Default|GetBox) false false)
      (Collision|SetCollisionEnabled (Variables|Default|GetBox) "NoCollision")
      (return self true))
    (else
      (return self false))))