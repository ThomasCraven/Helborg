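; Base Blueprint for player weapons that deals melee hit damage to enemies through a box overlap.
; AttackNow and DoNotAttack toggle the window in which overlaps count, with AttackNow also storing the weapon's top location as the attack start.
; Overlapped actors implementing BPI_Enemy receive base damage from the weapon's data asset via DamageMessage.
; Each hit also spawns force feedback at the player and a Niagara effect at the arrow component.
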(event OnComponentBeginOverlap(Box)
  (params (OverlappedComponent :type Primitive%20Component%20Object%20Reference) (OtherActor :type Actor%20Object%20Reference) (OtherComp :type Primitive%20Component%20Object%20Reference) (OtherBodyIndex :type Integer) (bFromSweep :type Boolean) (SweepResult :type Hit%20Result%20Structure%20%28by%20ref%29))
  (bind _data_asset (Variables|Default|GetData%20Asset))
  (if (Variables|Default|GetCanAttack?)
    (if (Utilities|DoesObjectImplementInterface OtherActor "/Game/SoulsLlike/Light/BluePrints/Interfaces/BPI_Enemy.BPI_Enemy_C")
      (Utilities|IsValid OtherActor
        (:Is%20Valid
          (Utilities|IsValid _data_asset
            (:Is%20Valid
              (Class|BPIEnemy|Damage(Message) OtherActor (Utilities|Struct|BreakStruct_DamageType (Variables|/Game/SoulsLlike/Light/DataAssets/BPD_WeaponData.BPD_WeaponData_C|GetDamageInfo _data_asset)))
              (ForceFeedback|SpawnForceFeedbackatLocation "/Game/SoulsLlike/Light/Inputs/Feedback/FF_VeryQuick.FF_VeryQuick" (Transformation|GetActorLocation (Game|GetPlayerCharacter 0)) "0, 0, 0" false 1.0 0.0 0)
              (Niagara|SpawnSystematLocation "/Game/SoulsLlike/Heavy/Systems/NS_WeaponHit.NS_WeaponHit" (Transformation|GetSocketLocation (Variables|Default|GetArrow) "None")))))))))

(event EventDoNotAttack
  (Variables|Default|SetCanAttack? false))

(event EventAttackNow
  (Variables|Default|SetCanAttack? true)
  (Variables|Default|SetStartAttack (Transformation|GetSocketLocation (Variables|Default|GetAttackTopLocasion) "")))

(event EventBeginPlay)

(fn ConstructionScript)