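; BP_BaseChest is a base interactable chest that opens once and spawns an item.
; BeginPlay caches the actor's starting transform.
; Initialise checks and clears the IsNotOpen flag, calls SpawnItem, then plays a timeline that lerps the ChestLid's world rotation to an open roll, keeping the starting pitch and yaw.
; When the timeline finishes, it calls NoCollision.
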(event EventBeginPlay
  (Variables|Default|SetStartTransform (Transformation|GetActorTransform)))

(event EventInitialise
  (bind _starttransform (Variables|Default|GetStartTransform))
  (Variables|Default|GetIsNotOpen?
    (:then
      (Variables|Default|SetIsNotOpen? false)
      (CallFunction|SpawnItem)
      (bind _alpha (Timeline|Timeline PlayFromStart)
        (:Update
          (Transformation|SetWorldRotation (Variables|Default|GetChestLid) (Math|Rotator|Lerp(Rotator) (.rotation (Variables|Default|GetStartTransform)) (Math|Rotator|MakeRotator (Variables|Default|GetOpen%28X%29%20Position) (.pitch (.rotation _starttransform)) (.yaw (.rotation _starttransform))) _alpha true) false false))
        (:Finished
          (CallFunction|NoCollision))))
    (:else)))

(fn ConstructionScript
  (|CallParentFunction))