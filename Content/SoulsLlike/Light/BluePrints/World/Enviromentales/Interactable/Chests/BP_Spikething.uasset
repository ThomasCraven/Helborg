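; Interactable in the Chests folder that swings two halves, Left and Right, open and spawns an item.
; BeginPlay caches the actor and both halves' starting transforms.
; When Initialise finds IsOpenUp set, it clears the flag, calls SpawnItem and runs a timeline lerping each half's yaw, then calls NoCollision.
; Otherwise, Initialise only sets the flag.
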(event EventBeginPlay
  (Variables|Default|SetStartTransform (Transformation|GetActorTransform))
  (Variables|Default|SetStartLeft (Transformation|GetRelativeTransform (Variables|Default|GetLeft)))
  (Variables|Default|SetStartRighrt (Transformation|GetRelativeTransform (Variables|Default|GetRight))))

(event EventInitialise
  (bind _startrighrt (Variables|Default|GetStartRighrt))
  (bind _startleft (Variables|Default|GetStartLeft))
  (Variables|Default|GetIsOpenUp?
    (:then
      (Variables|Default|SetIsOpenUp? false)
      (CallFunction|SpawnItem)
      (bind _alpha (Timeline|Timeline Play)
        (:Update
          (Transformation|SetRelativeRotation (Variables|Default|GetRight) (Math|Rotator|Lerp(Rotator) (.rotation (Variables|Default|GetStartRighrt)) (Math|Rotator|MakeRotator (.roll (.rotation _startrighrt)) (.pitch (.rotation _startrighrt)) (Variables|Default|GetB%20Z%20%28Yaw%29)) _alpha true) false false)
          (Transformation|SetRelativeRotation (Variables|Default|GetLeft) (Math|Rotator|Lerp(Rotator) (.rotation (Variables|Default|GetStartLeft)) (Math|Rotator|MakeRotator (.roll (.rotation _startleft)) (.pitch (.rotation _startleft)) (Variables|Default|GetB%20Z%20%28Yaw%29_0)) _alpha true) false false))
        (:Finished
          (CallFunction|NoCollision))))
    (:else
      (Variables|Default|SetIsOpenUp? true))))

(fn ConstructionScript
  (|CallParentFunction))