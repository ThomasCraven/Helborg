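; BP_RicketyLift is a lift actor that moves between its starting transform and a target MovetoLocal transform.
; BeginPlay caches the start transform, and each Initialise call uses the IsNotUp flag to play or reverse a Timeline.
; The Timeline's Alpha drives a transform lerp that moves the whole actor without sweeping for collision.
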(event EventBeginPlay
  (Variables|Default|SetStartTransform (Transformation|GetActorTransform)))

(event EventInitialise
  (Variables|Default|GetIsNotUp?
    (:then
      (Variables|Default|SetIsNotUp? false)
      (bind _alpha (Timeline|Timeline Play)
        (:Update
          (Transformation|SetActorTransform (Math|Transform|Lerp(Transform) (Variables|Default|GetStartTransform) (Variables|Default|GetMovetoLocal) _alpha)))))
    (:else
      (Variables|Default|SetIsNotUp? true)
      (Timeline|Timeline Reverse))))

(fn ConstructionScript
  (|CallParentFunction))