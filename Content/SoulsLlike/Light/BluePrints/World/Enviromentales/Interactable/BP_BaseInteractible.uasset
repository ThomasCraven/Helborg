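; BP_BaseInteractible is a base Blueprint for interactable world objects that show a pop-up prompt while overlapped.
; Its Box overlaps drive BPCPopUpUI to show and remove the prompt.
; Interact checks interaction and lock state, then calls the empty Initialise event and reports success.
; Helper functions spawn a configured item once with an amount, forward interaction to linked interactables, and disable the Box collision.
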(event OnComponentBeginOverlap(Box)
  (params (OverlappedComponent :type Primitive%20Component%20Object%20Reference) (OtherActor :type Actor%20Object%20Reference) (OtherComp :type Primitive%20Component%20Object%20Reference) (OtherBodyIndex :type Integer) (bFromSweep :type Boolean) (SweepResult :type Hit%20Result%20Structure%20%28by%20ref%29))
  (Variables|Default|GetCanShowPopup
    (:then
      (Default|PopUp (Variables|Default|GetBPC_PopUpUI) (Variables|Default|GetName) OtherActor 0 (Variables|Default|GetInteract%20Type) 0 OtherComp 0 self))
    (:else)))

(event OnComponentEndOverlap(Box)
  (params (OverlappedComponent :type Primitive%20Component%20Object%20Reference) (OtherActor :type Actor%20Object%20Reference) (OtherComp :type Primitive%20Component%20Object%20Reference) (OtherBodyIndex :type Integer))
  (Default|LeavePopUp (Variables|Default|GetBPC_PopUpUI) OtherActor OtherComp self))

(event Custom|Initialise)

(fn ConstructionScript)

(fn SpawnItem
  (LocalVariables|GetSpawned
    (:then
      _)
    (:else
      (bind _classtospawn (Variables|Default|GetClassTOSpawn)
        (:then
          (bind _returnvalue (Game|SpawnActorfromClass _classtospawn (Math|Transform|MakeTransform (Transformation|GetSocketLocation (Variables|Default|GetPick%20Spawn%20location) "None") "0, 0, 0" "1.000000,1.000000,1.000000") "AlwaysSpawn" "MultiplyWithRoot" 0 0))
          (Class|BPIInteract|AddAmount(Message) _returnvalue (Variables|Default|GetAmount))
          (LocalVariables|SetSpawned true))
        (:else))))
  (return))

(fn InteractwithOtherInteractable
  (for _array_element (Variables|Default|GetInract)
    (Utilities|IsValid _array_element
      (:Is%20Valid
        (Class|BPIInteract|Interact(Message) _array_element true 0 self)))))

(fn NoCollision
  (Collision|SetCollisionEnabled (Variables|Default|GetBox) "NoCollision"))

(fn Interact
  (params (HasIntracted? :type Boolean) (Player :type BP%20Base%20Souls%20Chap%20Object%20Reference) (InteractionItem :type Actor%20Object%20Reference))
  (if (and HasIntracted? (Variables|Default|GetCanIntract))
    (Variables|Default|GetIsLocked
      (:then)
      (:else
        (CallFunction|Initialise)
        (return self true)))))