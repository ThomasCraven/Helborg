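; BP_BasePortcullis is a base interactable portcullis door that moves vertically between its starting transform and a raised position.
; It caches its transform at BeginPlay, and each Initialise call toggles IsNotUp to play or reverse a timeline.
; The timeline's alpha lerps the actor toward a target that keeps the original X, Y, rotation and scale, with MoveUp as the absolute Z.
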(event EventBeginPlay
  (Variables|Default|SetStartTransform (Transformation|GetActorTransform)))

(event EventInitialise
  (bind _starttransform (Variables|Default|GetStartTransform))
  (Variables|Default|GetIsNotUp?
    (:then
      (Variables|Default|SetIsNotUp? false)
      (bind _alpha (Timeline|Timeline Play)
        (:Update
          (Transformation|SetActorTransform (Math|Transform|Lerp(Transform) (Variables|Default|GetStartTransform) (Math|Transform|MakeTransform (Math|Vector|MakeVector (.x (.location _starttransform)) (.y (.location _starttransform)) (Variables|Default|GetMoveUp)) (.rotation _starttransform) (.scale _starttransform)) _alpha)))))
    (:else
      (Variables|Default|SetIsNotUp? true)
      (Timeline|Timeline Reverse))))

(fn ConstructionScript
  (|CallParentFunction))