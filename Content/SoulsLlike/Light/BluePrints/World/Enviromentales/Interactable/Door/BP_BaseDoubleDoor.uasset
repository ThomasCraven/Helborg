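; Base interactable double door that swings its two leaves open and closed.
; BeginPlay caches the starting relative transforms of the Cube (left) and StaticMesh (right) leaves.
; Each Initialise call flips IsNotOpen and plays or reverses a Timeline.
; The Timeline lerps each leaf's rotation from its cached start to its own target yaw (LeftValue, RightValue), keeping pitch and roll, along the shortest path.
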(event EventBeginPlay
  (Variables|Default|SetStartLeft (Transformation|GetRelativeTransform (Variables|Default|GetCube)))
  (Variables|Default|SetStartRighrt (Transformation|GetRelativeTransform (Variables|Default|GetStaticMesh))))

(event EventInitialise
  (bind _startleft (Variables|Default|GetStartLeft))
  (bind _startrighrt (Variables|Default|GetStartRighrt))
  (Variables|Default|GetIsNotOpen?
    (:then
      (Variables|Default|SetIsNotOpen? false)
      (bind _alpha (Timeline|Timeline Play)
        (:Update
          (Transformation|SetRelativeRotation (Variables|Default|GetCube) (Math|Rotator|Lerp(Rotator) (.rotation (Variables|Default|GetStartLeft)) (Math|Rotator|MakeRotator (.roll (.rotation _startleft)) (.pitch (.rotation _startleft)) (Variables|Default|GetLeftValue)) _alpha true) false false)
          (Transformation|SetRelativeRotation (Variables|Default|GetStaticMesh) (Math|Rotator|Lerp(Rotator) (.rotation (Variables|Default|GetStartRighrt)) (Math|Rotator|MakeRotator (.roll (.rotation _startrighrt)) (.pitch (.rotation _startrighrt)) (Variables|Default|GetRightValue)) _alpha true) false false))))
    (:else
      (Variables|Default|SetIsNotOpen? true)
      (Timeline|Timeline Reverse))))

(fn ConstructionScript
  (|CallParentFunction))