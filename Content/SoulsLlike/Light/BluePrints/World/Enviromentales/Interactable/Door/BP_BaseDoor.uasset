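; Base interactable door for the world environment that swings open and closed.
; BeginPlay caches the starting transform, and Initialise calls its parent, then toggles the IsNotOpen flag to play a timeline forward or in reverse.
; Timeline updates lerp the Cube's world rotation along the shortest path from the starting yaw to the absolute RightRota yaw, preserving initial roll and pitch.
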(event EventBeginPlay
  (Variables|Default|SetStartTransform (Transformation|GetActorTransform)))

(event EventInitialise
  (bind _starttransform (Variables|Default|GetStartTransform))
  (|CallParentFunction)
  (Variables|Default|GetIsNotOpen?
    (:then
      (Variables|Default|SetIsNotOpen? false)
      (bind _alpha (Timeline|Timeline PlayFromStart)
        (:Update
          (Transformation|SetWorldRotation (Variables|Default|GetCube) (Math|Rotator|Lerp(Rotator) (.rotation (Variables|Default|GetStartTransform)) (Math|Rotator|MakeRotator (.roll (.rotation _starttransform)) (.pitch (.rotation _starttransform)) (Variables|Default|GetRightRota)) _alpha true) false false))))
    (:else
      (Variables|Default|SetIsNotOpen? true)
      (Timeline|Timeline ReverseFromEnd))))

(fn ConstructionScript
  (|CallParentFunction))