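; BP_Lether is an interactable lever that triggers another interactable and animates its stick between two positions.
; BeginPlay runs the parent logic and caches the stick's relative transform as the rest pose.
; Each Initialise call runs InteractWithOtherInteractable, then a FlipFlop alternately plays and reverses a Timeline.
; The Timeline lerps the stick's pitch from rest to a fixed angle, keeping its original roll and yaw.
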(event EventBeginPlay
  (|CallParentFunction)
  (Variables|Default|SetStickLocal (Transformation|GetRelativeTransform (Variables|Default|GetLetherStick))))

(event EventInitialise
  (bind _sticklocal (Variables|Default|GetStickLocal))
  (Utilities|FlowControl|Sequence
    (:then_0
      (CallFunction|InteractwithOtherInteractable))
    (:then_1
      (Utilities|FlowControl|FlipFlop
        (:A
          (bind _alpha (Timeline|Timeline Play)
            (:Update
              (Transformation|SetRelativeRotation (Variables|Default|GetLetherStick) (Math|Rotator|Lerp(Rotator) (.rotation (Variables|Default|GetStickLocal)) (Math|Rotator|MakeRotator (.roll (.rotation _sticklocal)) -1.5e+02 (.yaw (.rotation _sticklocal))) _alpha) false false))))
        (:B
          (Timeline|Timeline Reverse))))))

(fn ConstructionScript
  (|CallParentFunction))