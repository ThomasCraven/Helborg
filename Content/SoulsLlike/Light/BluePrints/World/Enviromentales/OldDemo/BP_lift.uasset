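; BP_lift is a lift actor that travels between a start point and a local offset, GotoLocal.
; An interact event or a BPI_Player actor entering its box toggles the direction, ignored while moving, and plays a door sound.
; A timeline lerps the actor's relative location forward or in reverse, using a start captured from the mesh's relative transform at BeginPlay.
; The Interact function itself only returns failure.
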(event OnComponentBeginOverlap(Box)
  (params (OverlappedComponent :type Primitive%20Component%20Object%20Reference) (OtherActor :type Actor%20Object%20Reference) (OtherComp :type Primitive%20Component%20Object%20Reference) (OtherBodyIndex :type Integer) (bFromSweep :type Boolean) (SweepResult :type Hit%20Result%20Structure%20%28by%20ref%29))
  (bind _start (Variables|Default|GetStart))
  (if (Utilities|DoesObjectImplementInterface OtherActor "/Game/SoulsLlike/Light/BluePrints/Interfaces/BPI_Player.BPI_Player_C")
    (if (Variables|Default|GetGoUp?)
      (if (Variables|Default|GetIsNotMoveing?)
        (CallFunction|Sounds)
        (Variables|Default|SetGoUp? false)
        (Variables|Default|SetIsNotMoveing? false)
        (bind _alpha (Timeline|Timeline Play)
          (:Update
            (Transformation|SetActorRelativeLocation (Math|Vector|Lerp(Vector) (.location _start) (+ (.location _start) (Variables|Default|GetGotoLocal)) _alpha)))
          (:Finished
            (Variables|Default|SetIsNotMoveing? true))))
      (elif (Variables|Default|GetIsNotMoveing?)
        (CallFunction|Sounds)
        (Variables|Default|SetGoUp? true)
        (Variables|Default|SetIsNotMoveing? false)
        (Timeline|Timeline Reverse)))))

(event Custom|Intract_1_1
  (params (HasIntracted? :type Boolean))
  (bind _start (Variables|Default|GetStart))
  (if HasIntracted?
    (if (Variables|Default|GetGoUp?)
      (if (Variables|Default|GetIsNotMoveing?)
        (CallFunction|Sounds)
        (Variables|Default|SetGoUp? false)
        (Variables|Default|SetIsNotMoveing? false)
        (bind _alpha (Timeline|Timeline Play)
          (:Update
            (Transformation|SetActorRelativeLocation (Math|Vector|Lerp(Vector) (.location _start) (+ (.location _start) (Variables|Default|GetGotoLocal)) _alpha)))
          (:Finished
            (Variables|Default|SetIsNotMoveing? true))))
      (elif (Variables|Default|GetIsNotMoveing?)
        (CallFunction|Sounds)
        (Variables|Default|SetGoUp? true)
        (Variables|Default|SetIsNotMoveing? false)
        (Timeline|Timeline Reverse)))))

(event EventBeginPlay
  (Variables|Default|SetStart (Transformation|GetRelativeTransform (Variables|Debug|GetStaticMeshComponent))))

(fn ConstructionScript)

(fn Sounds
  (Audio|PlaySoundatLocation "/Game/SoulsLlike/Light/Sound/Effects/SW_Dungeon_Door_Open_Wet_B.SW_Dungeon_Door_Open_Wet_B" (Transformation|GetSocketLocation (Variables|Debug|GetStaticMeshComponent) "None") "0, 0, 0" 1.0 1.0 0.0 0 0 0 0))

(fn Interact
  (params (HasIntracted? :type Boolean) (Player :type BP%20Base%20Souls%20Chap%20Object%20Reference))
  (return 0 false))