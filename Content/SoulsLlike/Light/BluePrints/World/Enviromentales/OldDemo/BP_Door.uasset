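; Interactable double door that swings both leaves open with a sound when the player interacts.
; Stores each leaf's starting relative transform, then a timeline lerps only the yaw toward per-side target angles along the shortest path.
; A box trigger shows or hides the interaction popup through BPI_Player.
; The Open flag blocks re-triggering only during the animation, resetting when it finishes; there is no closing logic.
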(event OnComponentBeginOverlap(Box)
  (params (OverlappedComponent :type Primitive%20Component%20Object%20Reference) (OtherActor :type Actor%20Object%20Reference) (OtherComp :type Primitive%20Component%20Object%20Reference) (OtherBodyIndex :type Integer) (bFromSweep :type Boolean) (SweepResult :type Hit%20Result%20Structure%20%28by%20ref%29))
  (if (and (Utilities|DoesObjectImplementInterface OtherActor "/Game/SoulsLlike/Light/BluePrints/Interfaces/BPI_Player.BPI_Player_C") (not (Variables|Default|GetOpen?)))
    (Class|BPIPlayer|Popup(Message) OtherActor (Variables|Default|GetIntract%20With) 0 "NewEnumerator0")
    (else
      (Class|BPIPlayer|LeavePopUp(Message) OtherActor))))

(event OnComponentEndOverlap(Box)
  (params (OverlappedComponent :type Primitive%20Component%20Object%20Reference) (OtherActor :type Actor%20Object%20Reference) (OtherComp :type Primitive%20Component%20Object%20Reference) (OtherBodyIndex :type Integer))
  (if (Utilities|DoesObjectImplementInterface OtherActor "/Game/SoulsLlike/Light/BluePrints/Interfaces/BPI_Player.BPI_Player_C")
    (Class|BPIPlayer|LeavePopUp(Message) OtherActor)))

(event EventIntract
  (params (HasIntracted? :type Boolean))
  (bind _leftstarttransform (Variables|Default|GetLeftStartTransform))
  (bind _rightstarttransform (Variables|Default|GetRightStartTransform))
  (if (and HasIntracted? (not (Variables|Default|GetOpen?)))
    (Variables|Default|SetOpen? true)
    (Audio|PlaySoundatLocation 0 "/Game/SoulsLlike/Light/Sound/Effects/SW_Dungeon_Door_Open_Wet_B.SW_Dungeon_Door_Open_Wet_B" (Transformation|GetSocketLocation (Variables|Default|GetLeft) "None") "0, 0, 0" 1.0 1.0 0.0 0 0 0 0)
    (bind _alpha (Timeline|Timeline Play)
      (:Update
        (Transformation|SetRelativeRotation (Variables|Default|GetRight) (Math|Rotator|Lerp(Rotator) (.rotation (Variables|Default|GetRightStartTransform)) (Math|Rotator|MakeRotator (.roll (.rotation _rightstarttransform)) (.pitch (.rotation _rightstarttransform)) (Variables|Default|GetRightRota)) _alpha true) false false)
        (Transformation|SetRelativeRotation (Variables|Default|GetLeft) (Math|Rotator|Lerp(Rotator) (.rotation (Variables|Default|GetLeftStartTransform)) (Math|Rotator|MakeRotator (.roll (.rotation _leftstarttransform)) (.pitch (.rotation _leftstarttransform)) (Variables|Default|GetLerttRota)) _alpha true) false false))
      (:Finished
        (Variables|Default|SetOpen? false)))))

(event EventBeginPlay
  (Variables|Default|SetRightStartTransform (Transformation|GetRelativeTransform (Variables|Default|GetRight)))
  (Variables|Default|SetLeftStartTransform (Transformation|GetRelativeTransform (Variables|Default|GetLeft))))

(fn ConstructionScript)