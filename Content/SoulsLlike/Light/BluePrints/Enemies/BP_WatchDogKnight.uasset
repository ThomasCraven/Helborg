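; BP_WatchDogKnight is a Watch Dog Knight enemy Blueprint that supplies the knight's attack against the player.
; AttackStart runs a zero-length multi sphere trace with a wide radius at the Arrow1 component on the Visibility channel.
; Each hit actor implementing BPI_Player receives AttackPlayerMessage with a fixed negative amount, with no de-duplication of hits.
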(event EventBeginPlay
  (|CallParentFunction) ; This node is disabled and will not be called.\nDrag off pins to build functionality.
)

(event Collision|EventActorBeginOverlap
  (params (OtherActor :type Actor%20Object%20Reference))
  (|CallParentFunction OtherActor) ; This node is disabled and will not be called.\nDrag off pins to build functionality.
)

(event EventTick
  (params (DeltaSeconds :type Float%20%28single-precision%29))
  (|CallParentFunction DeltaSeconds) ; This node is disabled and will not be called.\nDrag off pins to build functionality.
)

(event EventAttackStart
  (bind _arrow1 (Variables|Default|GetArrow1))
  (bind _returnvalue (Transformation|GetSocketLocation _arrow1 "None"))
  (bind (_outhits _returnvalue_2) (Collision|MultiSphereTraceByChannel _returnvalue _returnvalue 4e+02 "TraceTypeQuery1" false 0 "None"))
  (if _returnvalue_2
    (for _array_element _outhits
      (if (Utilities|DoesObjectImplementInterface (.HitActor (Collision|BreakHitResult _array_element)) "/Game/SoulsLlike/Light/BluePrints/Interfaces/BPI_Player.BPI_Player_C")
        (Class|BPIPlayer|AttackPlayer(Message) (.HitActor (Collision|BreakHitResult _array_element)) -4e+01)))))

(fn ConstructionScript
  (|CallParentFunction))