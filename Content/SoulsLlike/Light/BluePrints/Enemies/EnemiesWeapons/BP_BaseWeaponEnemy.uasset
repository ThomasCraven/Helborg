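; Base enemy melee weapon that damages the player with blade traces during attack windows.
; AttackNow enables attacking and starts a fast looping timer, evidently driving Damageplayer, while DoNotAttack disables attacking and clears it.
; Damageplayer sphere-traces between the blade's top and bottom markers on the Visibility channel, sending damage through BPI_Player to implementing actors.
; Hits are not de-duplicated, so damage can repeat within one swing.
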(event Custom|Damage%20player
  (bind (_outhits _returnvalue) (Collision|MultiSphereTraceByChannel (Transformation|GetSocketLocation (Variables|Default|GetAttackTopLocasion) "") (Transformation|GetSocketLocation (Variables|Default|GetAttackBottomLocasion) "") (Variables|Default|GetRadiusOfBlade) "TraceTypeQuery1" false 0 "None"))
  (if _returnvalue
    (for _array_element _outhits
      (if (and (Variables|Default|GetCanAttack?) (Utilities|DoesObjectImplementInterface (.HitActor (Collision|BreakHitResult _array_element)) "/Game/SoulsLlike/Light/BluePrints/Interfaces/BPI_Player.BPI_Player_C"))
        (Class|BPIPlayer|AttackPlayer(Message) (.HitActor (Collision|BreakHitResult _array_element)) (Variables|Default|GetDamage))))))

(event EventDoNotAttack
  (Variables|Default|SetCanAttack? false)
  (Utilities|Time|ClearandInvalidateTimerbyHandle (Variables|Default|GetAttackFrames)))

(event EventAttackNow
  (Variables|Default|SetCanAttack? true)
  (bind _returnvalue (Utilities|Time|SetTimerbyEvent (EventDispatchers|CreateEvent :!event Custom|Damage%20player) 0.01 true))
  (Variables|Default|SetAttackFrames _returnvalue))

(fn ConstructionScript)