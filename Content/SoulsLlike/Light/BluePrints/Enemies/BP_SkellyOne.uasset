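; BP_SkellyOne is a skeleton enemy Blueprint built on a parent enemy class, which plays its first attack montage once play begins.
; AttackStart and AttackEnd events message the weapon child actor to start and stop attacking.
; Its MakeSeleition override runs the parent logic, then sets the Skeletal array with its own Mesh in the last slot.
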(event EventBeginPlay
  (|CallParentFunction)
  (Animation|Montage|PlayMontage 0 "/Game/SoulsLlike/Heavy/Anims/Montages/AM_Attackone.AM_Attackone"))

(event EventAttackEnd
  (Class|BPIWeapon|DoNotAttack(Message) (Variables|/Script/Engine.ChildActorComponent|GetChildActor (Variables|Default|GetBP_BaseWeaponEnemy_Child))))

(event EventAttackStart
  (Class|BPIWeapon|AttackNow(Message) (Variables|/Script/Engine.ChildActorComponent|GetChildActor (Variables|Default|GetBP_BaseWeaponEnemy_Child))))

(fn ConstructionScript
  (|CallParentFunction))

(fn MakeSeleition
  (|CallParentFunction)
  (Variables|Default|SetSkeletal (Utilities|Array|MakeArray 0 0 0 0 0 0 0 0 0 0 0 0 0 0 0 0 0 0 0 0 0 0 0 0 0 0 0 0 0 (Variables|Character|GetMesh))))