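; Base enemy character for a Souls-like, handling health, combat, death and reset when the player dies.
; Exposed functions set patrol or chase speed and play random attack montages, returning their length.
; Damage updates a timed health bar, spawns blood, plays hit reactions that interrupt attacks, and opens a brief invulnerability window.
; Death plays a montage across the skeletal mesh array, with a timer leading to souls payout and actor destruction.
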(event Custom|AttackMon
  ;[0 0 0] Attack
  (if (not (Variables|Bool|GetIsDead?))
    (Audio|PlaySoundatLocation (Variables|Sound|GetAttackSound) (Transformation|GetSocketLocation (Variables|Default|GetCapsuleLockOn) "None") "0, 0, 0" 1.0 1.0 0.0 0 0 0 0)
    (Variables|/Script/Engine.CharacterMovementComponent|SetbUseControllerDesiredRotation (Variables|Character|GetCharacterMovement) false)
    (bind _array_element (Utilities|AccessSkeleton)
      (:LoopBody
        (Animation|Montage|PlayMontage _array_element (Variables|Anim|GetAttackMontageTwoPlay)
          (:then
            (Variables|Bool|SetIsStopAttack? false))
          (:OnCompleted
            (Variables|Bool|SetIsStopAttack? true :!label _label)
            (Default|CallEAttackEnd)
            (Variables|/Script/Engine.CharacterMovementComponent|SetbUseControllerDesiredRotation (Variables|Character|GetCharacterMovement) true))
          (:OnInterrupted
            (goto _label)))))))

(event Custom|DeathHit
  ;[0 0 0] Death
  (if (not (Variables|Bool|GetIsDead?))
    (CallFunction|SetWidgetVisibilityOff)
    (Variables|Bool|SetIsDead? true)
    (Variables|/Script/Engine.CharacterMovementComponent|SetbUseControllerDesiredRotation (Variables|Character|GetCharacterMovement) false)
    (Audio|PlaySoundatLocation "/Game/SoulsLlike/Light/Sound/Effects/SW_Miasma_003.SW_Miasma_003" (Transformation|GetSocketLocation (Variables|Default|GetCapsuleLockOn) "None") "0, 0, 0" 1.0 1.0 0.0 0 0 0 0)
    (bind _array_element (Utilities|AccessSkeleton)
      (:LoopBody
        (Animation|Montage|PlayMontage _array_element (Variables|Sound|GetDeathMontage)))
      (:Completed
        (bind _returnvalue (Utilities|Time|SetTimerbyEvent (EventDispatchers|CreateEvent :!event Death) (- (Animation|GetPlayLength (Variables|Sound|GetDeathMontage)) 0.5)))
        (Variables|info|SetDeathHandle _returnvalue)))))

(event EventChase
  (params (ChaseSpeed :type Float%20%28double-precision%29))
  ;[0 0 0] FoundPlayer
  (CallFunction|UpdateWalkSpeed (Variables|Value|GetChaseSpeed)))

(event EventFindPlayer
  (params (PlayerFound? :type Boolean))
  ;[0 0 0] FoundPlayer
  (Variables|Bool|SetPlayer%20Found? PlayerFound?)
  (CallFunction|SetWidgetVisibility))

(event EventDamage
  (params (DamageAmount :type Float%20%28double-precision%29))
  ;[0 0 0] Damage
  (bind _hasdamaged_ (CallFunction|ApplyDamage DamageAmount))
  (if _hasdamaged_
    (Audio|PlaySoundatLocation (Variables|Sound|GetHitSound) (Transformation|GetSocketLocation (Variables|Default|GetCapsuleLockOn) "None") "0, 0, 0" 1.0 1.0 0.0 0 0 0 0)
    (if (Variables|Bool|GetHasBlood?)
      (Niagara|SpawnSystematLocation (Variables|Anim|GetBloodTpye) (Transformation|GetSocketLocation (Variables|Default|GetCapsuleLockOn) "None"))
      (if (not (Variables|Bool|GetIsDead?))
        (Variables|Bool|SetIsStopAttack? true)
        (Default|CallEAttackEnd)
        (Animation|Montage|PlayMontage (Variables|Character|GetMesh) (RandomMontage|WitchHitMontage)
          (:then
            (Variables|Bool|SetEnemyState "NewEnumerator2"))
          (:OnCompleted
            (Variables|Bool|SetEnemyState "NewEnumerator0")
            (Variables|/Script/Engine.CharacterMovementComponent|SetbUseControllerDesiredRotation (Variables|Character|GetCharacterMovement) true)))))))

(event EventBeginPlay
  ;[0 0 0] SetUpEnemy
  (Variables|Value|SetStartTransform (Transformation|GetActorTransform))
  (bind _outactors (Actor|GetAllActorsOfClass "/Game/SoulsLlike/Light/BluePrints/Player/BP_BaseSoulsChap.BP_BaseSoulsChap_C"))
  (for _array_element _outactors
    (EventDispatchers|BindEventtoEDead _array_element (EventDispatchers|CreateEvent :!event PlayerDead)))
  (CallFunction|SetHealth)
  (CallFunction|MakeSeleition)
  (CallFunction|SetWidget))

(fn ConstructionScript)

(fn UpdateWalkSpeed
  (params (NewWalkSpeed :type Float%20%28double-precision%29))
  (Variables|/Script/Engine.CharacterMovementComponent|SetMaxWalkSpeed (Variables|Character|GetCharacterMovement) NewWalkSpeed))

(fn MakeSeleition
  (Variables|Anim|SetSkeletal (Utilities|Array|MakeArray (Variables|Character|GetMesh))))

(fn SetWidgetVisibilityon
  (Rendering|SetVisibility (Variables|Default|GetWidget) true false))

(fn SetWidgetVisibilityOff
  (Rendering|SetVisibility (Variables|Default|GetWidget) false false))

(fn SetWidgetVisibility
  (if (Variables|Bool|GetPlayer%20Found?)
    (Utilities|Time|SetTimerbyEvent (EventDispatchers|CreateEvent :!event SetWidgetVisibilityOff) 5.0)))

(fn SetHealth
  (bind _output_get (Variables|Value|SetCurrentHeealth (Variables|Value|GetMaxHealth)))
  (Default|CallEHEalthUpdate _output_get))

(fn SetWidget
  (bind _widget (Variables|Default|GetWidget)
    (:then
      (Default|Initialise (.AsWBP%20Health%20Bar%20Enemy (Utilities|Casting|CastToWBP_HealthBarEnemy (UserInterface|GetUserWidgetObject _widget))) self))
    (:else)))

(fn ApplyDamage
  (params (DamageAmount :type Float%20%28double-precision%29))
  (if (Variables|Bool|GetCanTakeDamage?)
    (bind _output_get (Variables|Value|SetCurrentHeealth (Math|Float|Clamp(Float) (+ DamageAmount (Variables|Value|GetCurrentHeealth)) 0.0 (Variables|Value|GetMaxHealth))))
    (Default|CallEHEalthUpdate _output_get)
    (if (<= _output_get 0.0)
      (CallFunction|DeathHit)
      (return false)
      (else
        (CallFunction|SetWidgetVisibilityon)
        (CallFunction|SetWidgetVisibility)
        (Variables|Bool|SetCanTakeDamage? false)
        (Utilities|Time|SetTimerbyEvent (EventDispatchers|CreateEvent :!event SetCanTakeDamage) 0.3)
        (return true)))
    (else
      (return false))))

(fn WitchAttackMontage
  (return (Utilities|Array|Get(acopy) (Variables|Anim|GetAttackMontage) (Math|Random|RandomInteger (Utilities|Array|Length (Variables|Anim|GetAttackMontage))))))

(fn Death
  (if (not (LocalVariables|GetDead))
    (LocalVariables|SetDead true)
    (Class|BPIPlayer|SendSouls(Message) (Game|GetPlayerCharacter 0) (.Souls (Utilities|Struct|BreakStruct_Enemy (Variables|Info|GetEenemyStruct))))
    (Niagara|SpawnSystematLocation "/Game/SoulsLlike/Heavy/Systems/NS_Souls.NS_Souls" (Transformation|GetSocketLocation (Variables|Collision|GetCapsuleComponent) "None"))
    (Actor|DestroyActor)))

(fn SetCanTakeDamage
  (Variables|Bool|SetCanTakeDamage? true))

(fn WitchHitMontage
  (bind _hitmontage (Variables|Anim|GetHitMontage))
  (return (Utilities|Array|Get(acopy) _hitmontage (Math|Random|RandomInteger (Utilities|Array|Length _hitmontage)))))

(fn PlayerDead
  (Transformation|SetActorRelativeTransform (Variables|Value|GetStartTransform) false true)
  (bind _output_get (Variables|Value|SetCurrentHeealth (Variables|Value|GetMaxHealth)))
  (Default|CallEHEalthUpdate _output_get)
  (Rendering|SetVisibility (Variables|Default|GetWidget) false false))

(fn Attack
  (bind _output_get (Variables|Anim|SetAttackMontageTwoPlay (RandomMontage|WitchAttackMontage)))
  (CallFunction|AttackMon)
  (return (Animation|GetPlayLength _output_get) self))

(fn FindPatrol
  (params (PatrolSpeed :type Float%20%28double-precision%29))
  (CallFunction|UpdateWalkSpeed (Variables|Value|GetPatrolSpeed))
  (return (Variables|Value|GetPatrol)))