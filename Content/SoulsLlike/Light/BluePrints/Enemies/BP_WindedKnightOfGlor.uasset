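; Winded Knight of Glor enemy, a child Blueprint built from modular skeletal mesh body and armor parts.
; It starts the AM_Attackone montage on BeginPlay, and AttackStart and AttackEnd toggle attacking on its child-actor weapon through messages.
; MakeSeleition extends the parent to gather the meshes into the Skeletal array.
; Death_1 runs the AccessSkeleton loop over that array with no per-mesh action, then destroys the actor.
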(event Custom|Death_1
  (Utilities|AccessSkeleton
    (:Completed
      (Actor|DestroyActor))))

(event EventBeginPlay
  (|CallParentFunction)
  (Animation|Montage|PlayMontage (Variables|Default|GetSkeletalMesh) "/Game/SoulsLlike/Heavy/Anims/Montages/AM_Attackone.AM_Attackone"))

(event EventAttackEnd
  (Class|BPIWeapon|DoNotAttack(Message) (Variables|/Script/Engine.ChildActorComponent|GetChildActor (Variables|Default|GetBP_BaseWeapon))))

(event EventAttackStart
  (Class|BPIWeapon|AttackNow(Message) (Variables|/Script/Engine.ChildActorComponent|GetChildActor (Variables|Default|GetBP_BaseWeapon))))

(fn ConstructionScript
  (|CallParentFunction))

(fn MakeSeleition
  (|CallParentFunction)
  (Variables|Default|SetSkeletal (Utilities|Array|MakeArray (Variables|Default|GetSkeletalMesh) (Variables|Default|GetSM_Gender_02_FacialHair) (Variables|Default|GetSM_All_11_KneeAttachment_Left) (Variables|Default|GetSM_Gender_05_ArmUpperLeft) (Variables|Default|GetSM_All_05_ShoulderAttachment_Right) (Variables|Default|GetSM_All_09_HipAttachment) (Variables|Default|GetSM_All_00_HeadCoverings_NoFacialHair) (Variables|Default|GetSM_Gender_11_LegRight) (Variables|Default|GetSM_Gender_12_LegLeft) (Variables|Default|GetSM_Gender_08_HandRight) (Variables|Default|GetSM_Gender_07_ArmLowerLeft) (Variables|Default|GetSM_Gender_06_ArmLowerRight) (Variables|Default|GetSM_All_12_Extra) (Variables|Default|GetSM_Gender_01_Eyebrows) (Variables|Default|GetSM_Gender_09_HandLeft) (Variables|Default|GetSM_All_00_HeadCoverings_NoHair) (Variables|Default|GetSM_All_08_ElbowAttachment_Left) (Variables|Default|GetSM_All_10_KneeAttachment_Right) (Variables|Default|GetSM_All_02_HeadAttachment_Helmet) (Variables|Default|GetSM_All_06_ShoulderAttachment_Left) (Variables|Default|GetSM_All_04_BackAttachment) (Variables|Default|GetSM_All_01_Hair) (Variables|Default|GetSM_All_03_ChestAttachment) (Variables|Default|GetSM_All_00_HeadCoverings_BaseHair) (Variables|Default|GetSM_All_07_ElbowAttachment_Right) (Variables|Default|GetSM_Gender_04_ArmUpperRight) (Variables|Default|GetSM_Gender_10_Hips) (Variables|Default|GetSM_Gender_00_Head) (Variables|Default|GetSM_All_02_HeadAttachment_Hair) (Variables|Character|GetMesh))))