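; BPC_PopUpUI is a component that relays interaction pop-up prompts to the player when something overlaps or leaves.
; PopUp and LeavePopUp check the capsule for the PlayerCapsule tag, then send show or leave messages through the BPI_Player interface.
; The show message carries name, icon, interact type, amount, data asset and overlapping actor.
; Interact is a debug stub that prints and returns success, and NewFunction is empty.
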(event EventBeginPlay)

(event EventTick
  (params (DeltaSeconds :type Float%20%28single-precision%29)))

(fn PopUp
  (params (Name :type Text) (Player :type Actor%20Object%20Reference) (Icon :type Texture%202D%20Object%20Reference) (Interact%20type :type E_InteractType%20Enum :default "NewEnumerator0") (Amount :type Integer) (Capsule :type Actor%20Component%20Object%20Reference) (DataAssetPopup :type BPD%20Item%20Data%20Object%20Reference) (OverlapingActor :type Actor%20Object%20Reference))
  (for _array_element (Variables|/Script/Engine.ActorComponent|GetComponentTags Capsule)
    (if (and (== _array_element "PlayerCapsule") (Utilities|DoesObjectImplementInterface Player "/Game/SoulsLlike/Light/BluePrints/Interfaces/BPI_Player.BPI_Player_C"))
      (Class|BPIPlayer|Popup(Message) Player Name Icon Interact%20type Amount DataAssetPopup OverlapingActor) ; show on UI
    )))

(fn LeavePopUp
  (params (Player :type Object%20Object%20Reference) (Target :type Actor%20Component%20Object%20Reference) (UnoverlapingActor :type Actor%20Object%20Reference))
  (Utilities|IsValid Target
    (:Is%20Valid
      (for _array_element (Variables|/Script/Engine.ActorComponent|GetComponentTags Target)
        (if (and (== _array_element "PlayerCapsule") (Utilities|DoesObjectImplementInterface Player "/Game/SoulsLlike/Light/BluePrints/Interfaces/BPI_Player.BPI_Player_C"))
          (Class|BPIPlayer|LeavePopUp(Message) Player UnoverlapingActor))))))

(fn NewFunction)

(fn Interact
  (params (HasIntracted? :type Boolean) (Player :type BP%20Base%20Souls%20Chap%20Object%20Reference))
  (if HasIntracted?
    (Development|PrintString "Heloo")
    (return 0 true)))