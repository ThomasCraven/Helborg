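; Player controller for the Souls-like game that sets up input, the main HUD and a custom cursor, and handles pausing.
; BeginPlay adds the locomotion and attack Enhanced Input contexts, enables full tick while paused and creates both widgets.
; The menu key flip-flops pause, cursor, event calls and player character messages; Unpause reuses the resume branch without advancing the flip-flop.
; Left click triggers the cursor widget's Select.
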(event Custom|Unpause
  (Variables|Default|SetbShowMouseCursor false)
  (Default|CallEUnpauseGame)
  (Widget|SetVisibility (Variables|/Game/SoulsLlike/Light/UI/WBP_Cursor.WBP_Cursor_C|GetSizeBoxCursor (Variables|Default|GetCurrentCursor)) "Hidden")
  (Game|SetGamePaused false)
  (Class|BPIPlayer|StartPlay(Message) (Game|GetPlayerCharacter 0)))

(event Input|EnhancedActionEvents|EnhancedInputActionIA_MainMenu
  (params (ActionValue :type Boolean) (ElapsedSeconds :type Float%20%28double-precision%29) (TriggeredSeconds :type Float%20%28double-precision%29) (InputAction :type Input%20Action%20Object%20Reference :default "/Game/SoulsLlike/Light/Inputs/InputAcsions/IA_MainMenu.IA_MainMenu"))
  (Utilities|FlowControl|FlipFlop
    (:A
      (Variables|Default|SetbShowMouseCursor true)
      (Default|CallEPauseGame)
      (Widget|SetVisibility (Variables|/Game/SoulsLlike/Light/UI/WBP_Cursor.WBP_Cursor_C|GetSizeBoxCursor (Variables|Default|GetCurrentCursor)) "Visible")
      (Game|SetGamePaused true)
      (Class|BPIPlayer|StopPlaying(Message) (Game|GetPlayerCharacter 0)))
    (:B
      (Variables|Default|SetbShowMouseCursor false)
      (Default|CallEUnpauseGame)
      (Widget|SetVisibility (Variables|/Game/SoulsLlike/Light/UI/WBP_Cursor.WBP_Cursor_C|GetSizeBoxCursor (Variables|Default|GetCurrentCursor)) "Hidden")
      (Game|SetGamePaused false)
      (Class|BPIPlayer|StartPlay(Message) (Game|GetPlayerCharacter 0)))))

(event Input|EnhancedActionEvents|EnhancedInputActionIA_LeftClick
  (params (ActionValue :type Boolean) (ElapsedSeconds :type Float%20%28double-precision%29) (TriggeredSeconds :type Float%20%28double-precision%29) (InputAction :type Input%20Action%20Object%20Reference :default "/Game/SoulsLlike/Light/Inputs/InputAcsions/IA_LeftClick.IA_LeftClick"))
  (Default|Select (Variables|Default|GetCurrentCursor)))

(event EventBeginPlay
  (bind _returnvalue (PlayerController|LocalPlayerSubsystems|GetEnhancedInputLocalPlayerSubsystem))
  (Utilities|IsValid _returnvalue ; Adds enhanced mapping context
    (:Is%20Valid
      (Variables|Default|SetbShouldPerformFullTickWhenPaused true)
      (Input|AddMappingContext _returnvalue "/Game/SoulsLlike/Light/Inputs/IMC_Locomotion.IMC_Locomotion" 0 "(bIgnoreAllPressedKeysUntilRelease=True,bForceImmediately=False,bNotifyUserSettings=False)")
      (Input|AddMappingContext _returnvalue "/Game/SoulsLlike/Light/Inputs/IMC_Attacks.IMC_Attacks" 0 "(bIgnoreAllPressedKeysUntilRelease=True,bForceImmediately=False,bNotifyUserSettings=False)")
      (bind _returnvalue_2 (UserInterface|CreateWidget "/Game/SoulsLlike/Light/UI/WBP_Cursor.WBP_Cursor_C"))
      (Class|PlayerController|SetMouseCursorWidget "Default" _returnvalue_2)
      (Widget|SetVisibility _returnvalue_2 "Hidden")
      (Variables|Default|SetCurrentCursor _returnvalue_2)
      (bind _returnvalue_3 (UserInterface|CreateWidget "/Game/SoulsLlike/Light/UI/WBP_Main.WBP_Main_C"))
      (Utilities|IsValid _returnvalue_3
        (:Is%20Valid
          (Variables|Default|SetTheHud _returnvalue_3)
          (UserInterface|Viewport|AddtoViewport _returnvalue_3 0))))))

(event EventShowCursor
  (Variables|Default|SetbShowMouseCursor true)
  (Widget|SetVisibility (Variables|/Game/SoulsLlike/Light/UI/WBP_Cursor.WBP_Cursor_C|GetSizeBoxCursor (Variables|Default|GetCurrentCursor)) "Visible"))

(event EventHideCursor
  (Variables|Default|SetbShowMouseCursor false)
  (Widget|SetVisibility (Variables|/Game/SoulsLlike/Light/UI/WBP_Cursor.WBP_Cursor_C|GetSizeBoxCursor (Variables|Default|GetCurrentCursor)) "Hidden"))

(event EventCursorClickButton
  (Default|Select (Variables|Default|GetCurrentCursor)))

(fn ConstructionScript)