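; Bonfire manager that tracks activated bonfires and sets the player's respawn point in a Souls-like game.
; On BeginPlay it caches the player through a message call, saves their location as the initial spawn point, and binds to respawn and bonfire activation events.
; Bonfire events update the spawn point from the bonfire's arrow and update the player's bonfire list component.
; Respawn events pass the latest spawn point to the player.
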(event Custom|Respawn
  ;[0 0 0] PlayerDeath
  (Default|SetRespawnLocasion (Variables|Default|GetBP_PlayerRef) (Variables|Default|GetSpawnPiont)) ; Function within player to set location to last activated bonfire
)

(event Custom|ActiveBonFire
  (params (Active :type Boolean) (Bonfire :type BP%20Bonfire%20Object%20Reference))
  (bind _bp_playerref (Variables|Default|GetBP_PlayerRef))
  (bind _bpc_bonfirelist (Variables|/Game/SoulsLlike/Light/BluePrints/Player/BP_BaseSoulsChap.BP_BaseSoulsChap_C|GetBPC_BonFireList _bp_playerref))
  ;[0 0 0] Activated bonfires
  (Utilities|Array|Add (Variables|Default|GetActiveBonfires) Bonfire)
  (Variables|Default|SetSpawnPiont (Transformation|GetSocketLocation (Variables|/Game/SoulsLlike/Light/BluePrints/World/BonFires/BP_Bonfire.BP_Bonfire_C|GetArrow Bonfire) "None"))
  (Utilities|IsValid _bp_playerref
    (:Is%20Valid
      (if Active
        (Default|AddtoActiveList _bpc_bonfirelist Bonfire)
        (else
          (Default|CreateBonFireList _bpc_bonfirelist))))))

(event EventBeginPlay
  (bind _returnvalue (Game|GetPlayerCharacter 0))
  ;[0 0 0] GetPlayer
  (Utilities|IsValid _returnvalue
    (:Is%20Valid
      (bind _player (Class|BPIPlayer|GetPlayer(Message) _returnvalue))
      (Variables|Default|SetBP_PlayerRef _player)
      (Variables|Default|SetSpawnPiont (Transformation|GetActorLocation (Variables|Default|GetBP_PlayerRef)))
      (EventDispatchers|BindEventtoERespawn (Variables|/Game/SoulsLlike/Light/BluePrints/Player/BP_BaseSoulsChap.BP_BaseSoulsChap_C|GetBPC_Respawn (Variables|Default|GetBP_PlayerRef)) (EventDispatchers|CreateEvent :!event Custom|Respawn))
      (for _array_element (Variables|Default|GetInMapBonfires)
        (Utilities|IsValid _array_element
          (:Is%20Valid
            (EventDispatchers|BindEventtoEBonFireActive _array_element (EventDispatchers|CreateEvent :!event Custom|ActiveBonFire))))))))

(fn ConstructionScript)