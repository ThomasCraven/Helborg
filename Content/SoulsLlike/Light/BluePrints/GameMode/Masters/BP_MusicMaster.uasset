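; BP_MusicMaster is a music manager Blueprint that plays background tracks as 2D sounds.
; One tick after BeginPlay it starts a fantasy track with a fade-in and sets a ChangeTime timer, storing its handle.
; PlayNextSound swaps a valid current sound for a second fixed track and sets another timer.
; Each FadeOut is followed immediately by Stop, so outgoing tracks cut rather than crossfade.
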(event Custom|PlayNextSound
  (bind _currentsound (Variables|Default|GetCurrentSound)
    (:then
      (Audio|Components|Audio|FadeOut _currentsound 0.5 0.0 "Linear" :!class /Script/Engine.AudioComponent)
      (Audio|Components|Audio|Stop _currentsound)
      (bind _returnvalue (Audio|CreateSound2D "/Game/SoulsLlike/Light/Sound/Music/DarkFantasy_Vol2_Arthur_Intensity_1.DarkFantasy_Vol2_Arthur_Intensity_1" 0.2 1.0 0.0 0))
      (Variables|Default|SetCurrentSound _returnvalue)
      (Audio|Components|Audio|FadeIn _returnvalue 0.5 1.0 0.0 "Linear" :!class /Script/Engine.AudioComponent)
      (bind _returnvalue_2 (Utilities|Time|SetTimerbyEvent (EventDispatchers|CreateEvent :!event Custom|PlayerStartingSound) (Variables|Default|GetChangeTime)))
      (Variables|Default|SetCurrentSoundHandle _returnvalue_2))
    (:else)))

(event Custom|PlayerStartingSound
  (bind _currentsound (Variables|Default|GetCurrentSound)
    (:then
      (Audio|Components|Audio|FadeOut _currentsound 0.5 0.0 "Linear" :!class /Script/Engine.AudioComponent)
      (Audio|Components|Audio|Stop _currentsound))
    (:else
      _))
  (bind _returnvalue (Audio|CreateSound2D "/Game/SoulsLlike/Light/Sound/Music/SW_Fantasy_Vol4_Descent_Intensity_2.SW_Fantasy_Vol4_Descent_Intensity_2" 0.2 1.0 0.0 0))
  (Variables|Default|SetCurrentSound _returnvalue)
  (Audio|Components|Audio|FadeIn _returnvalue 0.5 1.0 0.0 "Linear" :!class /Script/Engine.AudioComponent)
  (bind _returnvalue_2 (Utilities|Time|SetTimerbyEvent (EventDispatchers|CreateEvent :!event Custom|PlayNextSound) (Variables|Default|GetChangeTime)))
  (Variables|Default|SetCurrentSoundHandle _returnvalue_2))

(event EventBeginPlay
  (Utilities|FlowControl|DelayUntilNextTick)
  (CallFunction|PlayerStartingSound))

(fn ConstructionScript)