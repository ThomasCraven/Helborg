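; Player component for a Souls-like game that handles the death and respawn cycle.
; On death it stops play, sets the player state and a death gameplay tag, plays a slowed death montage on each skeletal mesh and starts timed delays.
; The death screen step broadcasts a death event and starts a respawn timer.
; Respawn broadcasts its event, restores weapon visibility, state, rotation and stats, and clears the tag; bonfire activation is an empty stub.
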(event Custom|PlayerDeath
  (bind _player (Class|BPIPlayer|GetPlayer(Message) (Components|GetOwner)))
  (bind _output_get (Variables|Default|SetPlayer _player))
  (Default|StopPlaying _output_get)
  (Variables|/Game/SoulsLlike/Light/BluePrints/Player/BP_BaseSoulsChap.BP_BaseSoulsChap_C|SetPlayersState (Variables|Default|GetPlayer) "NewEnumerator13")
  (GameplayTags|AddGameplayTag (Variables|/Game/SoulsLlike/Light/BluePrints/Player/BP_BaseSoulsChap.BP_BaseSoulsChap_C|GetPlayerTagsActions (Variables|Default|GetPlayer)) "(TagName=\"CharacterActoins.Busy.Death\")" :!class /Script/GameplayTags.BlueprintGameplayTagLibrary)
  (for _array_element (Variables|/Game/SoulsLlike/Light/BluePrints/Player/BP_BaseSoulsChap.BP_BaseSoulsChap_C|GetArrayOfSM (Variables|Default|GetPlayer))
    (Animation|Montage|PlayMontage _array_element "/Game/SoulsLlike/Heavy/Anims/Montages/AM_Death.AM_Death" 0.6 ; DaethAim
      (:then
        (bind _returnvalue (Utilities|Time|SetTimerbyEvent (EventDispatchers|CreateEvent :!event DeathScreen) 2.0)) ; Time to Death UI Screen
        (Variables|Default|SetTimeToDeathScreenHandle _returnvalue)))))

(fn Respawn
  (bind _player (Variables|Default|GetPlayer))
  (bind _player_2 (Variables|Default|GetPlayer))
  (Default|CallERespawn)
  (Default|VisWeapon _player_2)
  (Variables|/Game/SoulsLlike/Light/BluePrints/Player/BP_BaseSoulsChap.BP_BaseSoulsChap_C|SetPlayersState _player_2 "NewEnumerator3")
  (GameplayTags|RemoveGameplayTag (Variables|/Game/SoulsLlike/Light/BluePrints/Player/BP_BaseSoulsChap.BP_BaseSoulsChap_C|GetPlayerTagsActions _player_2) "(TagName=\"CharacterActoins.Busy.Death\")" :!class /Script/GameplayTags.BlueprintGameplayTagLibrary)
  (Default|SetBaseRotasion _player)
  (Default|Reset (Variables|/Game/SoulsLlike/Light/BluePrints/Player/BP_BaseSoulsChap.BP_BaseSoulsChap_C|GetBPC_Stats _player)))

(fn ActivateBonfire)

(fn DeathScreen
  (Default|CallEDeath)
  (Utilities|Time|SetTimerbyEvent (EventDispatchers|CreateEvent :!event Respawn) 3.0) ; Time To Respawn
)