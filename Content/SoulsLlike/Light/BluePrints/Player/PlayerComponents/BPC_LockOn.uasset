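; BPC_LockOn is a player component that toggles lock-on to a nearby enemy.
; A sphere trace gathers hit components on BPI_Enemy actors, and ClosestEnemy picks the one most aligned with the player's forward vector by dot product, not distance.
; A fast looping timer drives the lock, with TargetLockOn signaling rotation toward the target while it is valid and within radius.
; StopLockOn clears the timer and targets, then signals the release.
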(fn LookforLockon
  (bind _returnvalue (Game|GetPlayerCharacter 0))
  (bind _returnvalue_2 (Transformation|GetActorLocation _returnvalue))
  (bind (_outhits _returnvalue_3) (Collision|MultiSphereTraceForObjects _returnvalue_2 _returnvalue_2 (Variables|Default|GetRadiusLockOn) (Utilities|Array|MakeArray "ObjectTypeQuery7") false 0 "None")) ; When used looks for enemies within a radius to lock onto
  (for _array_element _outhits
    (if (and _returnvalue_3 (Utilities|DoesObjectImplementInterface (.HitActor (Collision|BreakHitResult _array_element)) "/Game/SoulsLlike/Light/BluePrints/Interfaces/BPI_Enemy.BPI_Enemy_C"))
      (Utilities|Array|Add (Variables|Default|GetTargets) (.HitComponent (Collision|BreakHitResult _array_element)))))
  (return (CallFunction|ClosestEnemy (Variables|Default|GetTargets))))

(fn ClosestEnemy
  (params (Array :type Array%20of%20Primitive%20Component%20Object%20References))
  (bind _returnvalue (Game|GetPlayerCharacter 0))
  (for _array_element Array ; Cycles through the enemies to find the closest
    (Math|Float|CompareFloat (Math|Vector|DotProduct (Transformation|GetActorForwardVector _returnvalue) (Math|Rotator|GetRotationXVector (Math|Rotator|FindLookatRotation (Transformation|GetActorLocation _returnvalue) (Transformation|GetSocketLocation _array_element "None")))) (Variables|Default|GetCompare%20With)
      (:>
        (Variables|Default|SetCompare%20With (Math|Vector|DotProduct (Transformation|GetActorForwardVector _returnvalue) (Math|Rotator|GetRotationXVector (Math|Rotator|FindLookatRotation (Transformation|GetActorLocation _returnvalue) (Transformation|GetSocketLocation _array_element "None")))))
        (LocalVariables|SetClosestTarget _array_element))))
  (Variables|Default|SetCompare%20With 0.0)
  (return (LocalVariables|GetClosestTarget)))

(fn StartLockon
  (if (not (Variables|Default|GetIsLocker?))
    (Variables|Default|SetIsLocker? true)
    (bind _target (CallFunction|LookforLockon))
    (Utilities|IsValid _target
      (:Is%20Valid
        (Variables|Default|SetTarget _target)
        (bind _returnvalue (Utilities|Time|SetTimerbyEvent (EventDispatchers|CreateEvent :!event TargetLockon) 0.001 true)) ; Tells the player camera to lock onto this location
        (Variables|Default|SetLockOnHandle _returnvalue))
      (:Is%20Not%20Valid
        (CallFunction|StopLockon)))
    (else
      (CallFunction|StopLockon))))

(fn TargetLockon
  (bind _target (Variables|Default|GetTarget) ; Is target dead
    (:then
      (if (not (> (Math|Vector|Distance(Vector) (Transformation|GetActorLocation (Game|GetPlayerCharacter 0)) (Transformation|GetSocketLocation _target "None")) (Variables|Default|GetRadiusLockOn))) ; lock on radius
        (Default|CallESetRotaionLockon :Target (Variables|Default|GetTarget))
        (else
          (CallFunction|StopLockon))))
    (:else
      (CallFunction|StopLockon))))

(fn StopLockon
  (Utilities|Time|ClearandInvalidateTimerbyHandle (Variables|Default|GetLockOnHandle))
  (Variables|Default|SetIsLocker? false)
  (Variables|Default|SetTarget 0)
  (Utilities|Array|Clear (Variables|Default|GetTargets))
  (Default|CallEStopLockon))