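; Player component that handles using the currently selected consumable from the Souls-like player's inventory component.
; UseItem starts a short cooldown timer on every call, then checks validity, quantity and the can-use flag before hiding the weapon and removing one item.
; Successful removal shows the consumable and plays a throw or drink animation by item type; failed removal triggers the player's item-failed response.
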(event EventBeginPlay)

(event EventTick
  (params (DeltaSeconds :type Float%20%28single-precision%29)))

(fn UseItem
  (params (Player :type BP%20Base%20Souls%20Chap%20Object%20Reference))
  (Variables|Default|SetPlayer Player)
  (bind _returnvalue (Utilities|Time|SetTimerbyEvent (EventDispatchers|CreateEvent :!event UseItemCooldown) 0.5))
  (Variables|Default|SetUseItemColldownHandle _returnvalue)
  (if (Math|Boolean|ANDBoolean (Utilities|IsValid (.Consumable (Utilities|Struct|BreakStruct_ConsumableQuantity (Variables|/Game/SoulsLlike/Light/BluePrints/Player/PlayerComponents/BPC_Inventory.BPC_Inventory_C|GetCurrentSelectedConsumable (Variables|/Game/SoulsLlike/Light/BluePrints/Player/BP_BaseSoulsChap.BP_BaseSoulsChap_C|GetBPC_Inventory (Variables|Default|GetPlayer)))))) (> (.Quantity (Utilities|Struct|BreakStruct_ConsumableQuantity (Variables|/Game/SoulsLlike/Light/BluePrints/Player/PlayerComponents/BPC_Inventory.BPC_Inventory_C|GetCurrentSelectedConsumable (Variables|/Game/SoulsLlike/Light/BluePrints/Player/BP_BaseSoulsChap.BP_BaseSoulsChap_C|GetBPC_Inventory (Variables|Default|GetPlayer))))) 0) (Variables|Default|GetCanUseItem))
    (Default|HiddenWeapon (Variables|Default|GetPlayer))
    (Variables|Default|SetCanUseItem false)
    (bind _hasitems (Default|RemoveConsumables (Variables|/Game/SoulsLlike/Light/BluePrints/Player/BP_BaseSoulsChap.BP_BaseSoulsChap_C|GetBPC_Inventory (Variables|Default|GetPlayer)) 1 (Variables|/Game/SoulsLlike/Light/BluePrints/Player/PlayerComponents/BPC_Inventory.BPC_Inventory_C|GetCurrentSelectedConsumable (Variables|/Game/SoulsLlike/Light/BluePrints/Player/BP_BaseSoulsChap.BP_BaseSoulsChap_C|GetBPC_Inventory (Variables|Default|GetPlayer)))))
    (if _hasitems
      (Default|UnhiddenConsumable (Variables|Default|GetPlayer) (.Class (Utilities|Struct|BreakStruct_Consumable (Variables|/Game/SoulsLlike/Light/DataAssets/BPD_ConsumableData.BPD_ConsumableData_C|GetConsumableInfo (.Consumable (Utilities|Struct|BreakStruct_ConsumableQuantity (Variables|/Game/SoulsLlike/Light/BluePrints/Player/PlayerComponents/BPC_Inventory.BPC_Inventory_C|GetCurrentSelectedConsumable (Variables|/Game/SoulsLlike/Light/BluePrints/Player/BP_BaseSoulsChap.BP_BaseSoulsChap_C|GetBPC_Inventory (Variables|Default|GetPlayer)))))))))
      (switch Utilities|FlowControl|Switch|SwitchonE_ConsumableType (.Type (Utilities|Struct|BreakStruct_Consumable (Variables|/Game/SoulsLlike/Light/DataAssets/BPD_ConsumableData.BPD_ConsumableData_C|GetConsumableInfo (.Consumable (Utilities|Struct|BreakStruct_ConsumableQuantity (Variables|/Game/SoulsLlike/Light/BluePrints/Player/PlayerComponents/BPC_Inventory.BPC_Inventory_C|GetCurrentSelectedConsumable (Variables|/Game/SoulsLlike/Light/BluePrints/Player/BP_BaseSoulsChap.BP_BaseSoulsChap_C|GetBPC_Inventory (Variables|Default|GetPlayer))))))))
        (:NewEnumerator1
          (Default|ThrowAnim (Variables|Default|GetPlayer)))
        (:NewEnumerator2
          (Default|DrinkAnim (Variables|Default|GetPlayer))))
      (else
        (Default|ItemFailed (Variables|Default|GetPlayer))))))

(fn UseItemCooldown
  (Variables|Default|SetCanUseItem true))