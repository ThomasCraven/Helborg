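; Player combat component for a Souls-like game that handles light attack, heavy attack and shield-raise input.
; Attacks require an available action, a valid weapon and a stamina update, then play montages on every player mesh while tagged as attacking.
; AttackStart and AttackEnd message the weapon's child actor to toggle attacking.
; Holding the shield switches player state and slows walk speed, restoring both on release.
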(event Input|EnhancedActionEvents|EnhancedInputActionIA_ShieldUp
  (params (ActionValue :type Boolean) (ElapsedSeconds :type Float%20%28double-precision%29) (TriggeredSeconds :type Float%20%28double-precision%29) (InputAction :type Input%20Action%20Object%20Reference :default "/Game/SoulsLlike/Light/Inputs/InputAcsions/IA_ShieldUp.IA_ShieldUp"))
  (bind _player (Variables|Default|GetPlayer))
  (bind _charactermovement (Variables|/Script/Engine.Character|GetCharacterMovement _player))
  ;[0.15 0.15 0.15 0.5] ShieldUp
  (:Triggered
    (Variables|/Game/SoulsLlike/Light/BluePrints/Player/BP_BaseSoulsChap.BP_BaseSoulsChap_C|SetPlayersState _player "NewEnumerator11" :!label _label)
    (Variables|/Script/Engine.CharacterMovementComponent|SetMaxWalkSpeed _charactermovement 3e+02))
  (:Started
    (goto _label))
  (:Canceled
    (Variables|/Game/SoulsLlike/Light/BluePrints/Player/BP_BaseSoulsChap.BP_BaseSoulsChap_C|SetPlayersState _player "NewEnumerator3" :!label _label_2)
    (Variables|/Script/Engine.CharacterMovementComponent|SetMaxWalkSpeed _charactermovement 6e+02))
  (:Completed
    (goto _label_2)))

(event Input|EnhancedActionEvents|EnhancedInputActionIA_HeaveyAttack
  (params (ActionValue :type Boolean) (ElapsedSeconds :type Float%20%28double-precision%29) (TriggeredSeconds :type Float%20%28double-precision%29) (InputAction :type Input%20Action%20Object%20Reference :default "/Game/SoulsLlike/Light/Inputs/InputAcsions/IA_HeaveyAttack.IA_HeaveyAttack"))
  ;[0.15 0.15 0.15 0.5] HeavyAttack
  (bind _player (Class|BPIPlayer|GetPlayer(Message) (Components|GetOwner)))
  (Variables|Default|SetPlayer _player)
  (if (and (Default|CanMakeAcsoin (Variables|Default|GetPlayer)) (Utilities|IsValid (Variables|/Game/SoulsLlike/Light/BluePrints/Player/BP_BaseSoulsChap.BP_BaseSoulsChap_C|GetCurrentWeapon (Variables|Default|GetPlayer))))
    (Default|VisWeapon (Variables|Default|GetPlayer))
    (bind _success (Default|StanimaUpdata (Variables|/Game/SoulsLlike/Light/BluePrints/Player/BP_BaseSoulsChap.BP_BaseSoulsChap_C|GetBPC_Stats (Variables|Default|GetPlayer)) (Utilities|Struct|BreakStruct_PlayerStats (Variables|/Game/SoulsLlike/Light/BluePrints/Player/BP_BaseSoulsChap.BP_BaseSoulsChap_C|GetPlayerInfo (Variables|Default|GetPlayer)))))
    (if _success
      (for _array_element (Variables|/Game/SoulsLlike/Light/BluePrints/Player/BP_BaseSoulsChap.BP_BaseSoulsChap_C|GetArrayOfSM (Variables|Default|GetPlayer))
        (Animation|Montage|PlayMontage _array_element "/Game/SoulsLlike/Heavy/Anims/Montages/AM_Heavytattck.AM_Heavytattck"
          (:then
            (GameplayTags|AddGameplayTag (Variables|/Game/SoulsLlike/Light/BluePrints/Player/BP_BaseSoulsChap.BP_BaseSoulsChap_C|GetPlayerTagsActions (Variables|Default|GetPlayer)) "(TagName=\"CharacterActoins.Busy.Attacking\")" :!class /Script/GameplayTags.BlueprintGameplayTagLibrary))
          (:OnCompleted
            (GameplayTags|RemoveGameplayTag (Variables|/Game/SoulsLlike/Light/BluePrints/Player/BP_BaseSoulsChap.BP_BaseSoulsChap_C|GetPlayerTagsActions (Variables|Default|GetPlayer)) "(TagName=\"CharacterActoins.Busy.Attacking\")" :!class /Script/GameplayTags.BlueprintGameplayTagLibrary)))))))

(event Input|EnhancedActionEvents|EnhancedInputActionIA_lightAttack
  (params (ActionValue :type Boolean) (ElapsedSeconds :type Float%20%28double-precision%29) (TriggeredSeconds :type Float%20%28double-precision%29) (InputAction :type Input%20Action%20Object%20Reference :default "/Game/SoulsLlike/Light/Inputs/InputAcsions/IA_lightAttack.IA_lightAttack"))
  ;[0.15 0.15 0.15 0.5] LightAttack
  (bind _player (Class|BPIPlayer|GetPlayer(Message) (Components|GetOwner)))
  (Variables|Default|SetPlayer _player)
  (if (and (Default|CanMakeAcsoin (Variables|Default|GetPlayer)) (Utilities|IsValid (Variables|/Game/SoulsLlike/Light/BluePrints/Player/BP_BaseSoulsChap.BP_BaseSoulsChap_C|GetCurrentWeapon (Variables|Default|GetPlayer))))
    (Default|VisWeapon (Variables|Default|GetPlayer))
    (bind _success (Default|StanimaUpdata (Variables|/Game/SoulsLlike/Light/BluePrints/Player/BP_BaseSoulsChap.BP_BaseSoulsChap_C|GetBPC_Stats (Variables|Default|GetPlayer)) (Utilities|Struct|BreakStruct_PlayerStats (Variables|/Game/SoulsLlike/Light/BluePrints/Player/BP_BaseSoulsChap.BP_BaseSoulsChap_C|GetPlayerInfo (Variables|Default|GetPlayer)))))
    (if _success
      (for _array_element (Variables|/Game/SoulsLlike/Light/BluePrints/Player/BP_BaseSoulsChap.BP_BaseSoulsChap_C|GetArrayOfSM (Variables|Default|GetPlayer))
        (Animation|Montage|PlayMontage _array_element "/Game/SoulsLlike/Heavy/Anims/Montages/AM_lightattck.AM_lightattck"
          (:then
            (GameplayTags|AddGameplayTag (Variables|/Game/SoulsLlike/Light/BluePrints/Player/BP_BaseSoulsChap.BP_BaseSoulsChap_C|GetPlayerTagsActions (Variables|Default|GetPlayer)) "(TagName=\"CharacterActoins.Busy.Attacking\")" :!class /Script/GameplayTags.BlueprintGameplayTagLibrary))
          (:OnCompleted
            (GameplayTags|RemoveGameplayTag (Variables|/Game/SoulsLlike/Light/BluePrints/Player/BP_BaseSoulsChap.BP_BaseSoulsChap_C|GetPlayerTagsActions (Variables|Default|GetPlayer)) "(TagName=\"CharacterActoins.Busy.Attacking\")" :!class /Script/GameplayTags.BlueprintGameplayTagLibrary)))))))

(event EventAttackEnd
  ;[0.15 0.15 0.15 0.5] AttackEndandStart
  (Class|BPIWeapon|DoNotAttack(Message) (Variables|/Script/Engine.ChildActorComponent|GetChildActor (Variables|/Game/SoulsLlike/Light/BluePrints/Player/BP_BaseSoulsChap.BP_BaseSoulsChap_C|GetBP_BaseWeapon (Variables|Default|GetPlayer)))))

(event EventAttackStart
  ;[0.15 0.15 0.15 0.5] AttackEndandStart
  (Class|BPIWeapon|AttackNow(Message) (Variables|/Script/Engine.ChildActorComponent|GetChildActor (Variables|/Game/SoulsLlike/Light/BluePrints/Player/BP_BaseSoulsChap.BP_BaseSoulsChap_C|GetBP_BaseWeapon (Variables|Default|GetPlayer)))))