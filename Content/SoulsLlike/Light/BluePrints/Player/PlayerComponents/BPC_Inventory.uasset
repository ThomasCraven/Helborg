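; Player inventory component for a Souls-like game that tracks souls, weapons, shields, armor, charms and consumable stacks.
; Items are typed data assets that ItemAdded casts and routes to per-type add functions, with separate owned and equipped storage.
; Equip, unequip and cycling functions update arrays, slots and indices, then fire event dispatchers to refresh UI and HUD.
; The inventory input flip-flops between opening the UI with a cursor and returning to play.
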(event Input|EnhancedActionEvents|EnhancedInputActionIA_Inventory
  (params (ActionValue :type Boolean) (ElapsedSeconds :type Float%20%28double-precision%29) (TriggeredSeconds :type Float%20%28double-precision%29) (InputAction :type Input%20Action%20Object%20Reference :default "/Game/SoulsLlike/Light/Inputs/InputAcsions/IA_Inventory.IA_Inventory"))
  (bind _returnvalue (Game|GetPlayerCharacter 0))
  (bind _returnvalue_2 (Game|GetPlayerController 0))
  ;[0 0 0] Open and close Inventory
  (Utilities|FlowControl|FlipFlop ; OpenClose
    (:A
      (Class|BPIPlayer|StopPlaying(Message) _returnvalue) ; StopInputsAndUIMode
      (Class|BPIController|ShowCursor(Message) _returnvalue_2)
      (Default|CallEOpen) ; OpenUI
      (Default|CallEUpdateInventory self) ; ReFreshUI
    )
    (:B
      (Class|BPIPlayer|StartPlay(Message) _returnvalue) ; PlayMode
      (Default|CallEClear) ; CloseUI
      (Class|BPIController|HideCursor(Message) _returnvalue_2))))

(event EventBeginPlay
  ;[0 0 0] Initialise
  (bind _player (Variables|Default|GetPlayer)
    (:then
      (EventDispatchers|BindEventtoEPickUpInfo _player (EventDispatchers|CreateEvent :!event ItemAdded)))
    (:else)))

(fn AddSouls
  (params (SoulsAdded :type Integer) (Player :type BP%20Base%20Souls%20Chap%20Object%20Reference))
  (Variables|Default|SetPlayer Player)
  (if (not (< (+ SoulsAdded (Variables|Default|GetCurrent%20Souls)) 0))
    (bind _output_get (Variables|Default|SetCurrent%20Souls (+ SoulsAdded (Variables|Default|GetCurrent%20Souls))))
    (Default|CallESoulsUpdate _output_get)))

(fn WeaponSeleced
  (params (WeaponAddIndex :type Integer))
  (bind _weaponsequiped (Variables|Default|GetWeaponsEquiped))
  (bind _weaponsequiped_2 (Variables|Default|GetWeaponsEquiped))
  (bind _weaponsequiped_3 (Variables|Default|GetWeaponsEquiped))
  (bind _returnvalue (Utilities|Array|LastIndex _weaponsequiped))
  (bind _output (Utilities|Array|Get(acopy) _weaponsequiped_3))
  ;[0 0 0] Switch Weapon Index
  (Variables|Default|SetWeaponIndex (+ WeaponAddIndex (Variables|Default|GetWeaponIndex)))
  (if (> (Variables|Default|GetWeaponIndex) (Utilities|Array|LastIndex (Variables|Default|GetWeaponsEquiped)))
    ;[0 0 0] Set Selected Weapon
    ;;[0.3802 0.3802 0.3802] Set to first index
    (Variables|Default|SetWeaponIndex 0)
    (Utilities|IsValid _output
      (:Is%20Valid
        (Default|CallESwitchWeapon _output))
      (:Is%20Not%20Valid
        (Utilities|Array|RemoveIndex _weaponsequiped_3)
        (Default|CallESwitchWeapon (Utilities|Array|Get(acopy) _weaponsequiped_3))))
    (else
      ;;[0.3802 0.3802 0.3802] Cycle though Array
      (if (< (Variables|Default|GetWeaponIndex) 0)
        (bind _output_get (Variables|Default|SetWeaponIndex _returnvalue))
        (Utilities|IsValid (Utilities|Array|Get(acopy) _weaponsequiped _returnvalue)
          (:Is%20Valid
            (Default|CallESwitchWeapon))
          (:Is%20Not%20Valid
            (Utilities|Array|RemoveIndex _weaponsequiped _output_get)
            (Default|CallESwitchWeapon (Utilities|Array|Get(acopy) _weaponsequiped (Variables|Default|GetWeaponIndex)))))
        (else
          ;;[0.3802 0.3802 0.3802] SetLastArray
          (Utilities|IsValid (Utilities|Array|Get(acopy) (Variables|Default|GetWeaponsEquiped) (Variables|Default|GetWeaponIndex))
            (:Is%20Valid
              (Default|CallESwitchWeapon (Utilities|Array|Get(acopy) (Variables|Default|GetWeaponsEquiped) (Variables|Default|GetWeaponIndex))))
            (:Is%20Not%20Valid
              (Utilities|Array|RemoveIndex _weaponsequiped_2 (Variables|Default|GetWeaponIndex))
              (Default|CallESwitchWeapon (Utilities|Array|Get(acopy) _weaponsequiped_2)))))))))

(fn AddConsumables
  (params (ConsumableData :type BPD%20Consumable%20Data%20Object%20Reference) (ConsumableQuantity :type Integer))
  ;[0 0 0] AddConsumables
  (LocalVariables|SetConsumable ConsumableData)
  (LocalVariables|SetAmount ConsumableQuantity)
  (for (_array_element _array_index) (Variables|Default|GetConsumableQuantity)
    ;[0 0 0] AddToItemAmount
    (if (not (and (== (.Consumable (Utilities|Struct|BreakStruct_ConsumableQuantity _array_element)) (LocalVariables|GetConsumable)) (> (.Quantity (Utilities|Struct|BreakStruct_ConsumableQuantity _array_element)) 0))) ; Is Item in inventory already
      (LocalVariables|SetIsNew? true)
      (else
        (Variables|Default|SetArray%20Index _array_index)
        (Variables|Default|SetNewItemAmount (+ (.Quantity (Utilities|Struct|BreakStruct_ConsumableQuantity _array_element)) (LocalVariables|GetAmount)))
        (Utilities|Array|SetArrayElem (Variables|Default|GetConsumableQuantity) (Variables|Default|GetArray%20Index) (Utilities|Struct|MakeStruct_ConsumableQuantity (LocalVariables|GetConsumable) (Variables|Default|GetNewItemAmount))) ; Add to Quantity Consumable
        (LocalVariables|SetIsNew? false)
        ;[0 0 0] Check If is Equiped already
        (for (_array_element_2 _array_index_2) (Variables|Default|GetConsumableQuantityEquiped) ; Verifies whether the consumable is already equipped.\nUsed to prevent multiple instances of the same item being active at once
          (if (not (not (and (== (.Consumable (Utilities|Struct|BreakStruct_ConsumableQuantity _array_element_2)) (LocalVariables|GetConsumable)) (> (.Quantity (Utilities|Struct|BreakStruct_ConsumableQuantity _array_element_2)) 0)))) ; Is Item in inventory already
            (Variables|Default|SetConsumableEquipedIndex _array_index_2)
            (Variables|Default|SetNewItemAmount (+ (.Quantity (Utilities|Struct|BreakStruct_ConsumableQuantity _array_element_2)) (LocalVariables|GetAmount)))
            (Utilities|Array|SetArrayElem (Variables|Default|GetConsumableQuantityEquiped) (Variables|Default|GetConsumableEquipedIndex) (Utilities|Struct|MakeStruct_ConsumableQuantity (LocalVariables|GetConsumable) (Variables|Default|GetNewItemAmount))) ; Set Item Amount in inventory
            (Default|CallESwitchComsumable (.Icon (Utilities|Struct|BreakStruct_ItemHeader (Variables|/Game/SoulsLlike/Light/DataAssets/BPD_ItemData.BPD_ItemData_C|GetItemInfo (.Consumable (Utilities|Struct|BreakStruct_ConsumableQuantity _array_element_2))))) (.Name (Utilities|Struct|BreakStruct_ItemHeader (Variables|/Game/SoulsLlike/Light/DataAssets/BPD_ItemData.BPD_ItemData_C|GetItemInfo (.Consumable (Utilities|Struct|BreakStruct_ConsumableQuantity _array_element_2))))) (.Quantity (Utilities|Struct|BreakStruct_ConsumableQuantity _array_element_2)))
            (Default|SetEquip (.Consumable (Utilities|Struct|BreakStruct_ConsumableQuantity _array_element_2)) true)
            (return true))))))
  ;[0 0 0] AddNewItem
  (if (LocalVariables|GetIsNew?) ; Is Item New
    (Variables|Default|SetNewItemAmount (LocalVariables|GetAmount))
    (Utilities|Array|Add (Variables|Default|GetConsumableQuantity) (Utilities|Struct|MakeStruct_ConsumableQuantity (LocalVariables|GetConsumable) (LocalVariables|GetAmount))) ; AddNew Consumable and quantity
    (Default|CallEEquiped self)
    (LocalVariables|SetIsNew? false)
    (if (<= (Utilities|Array|Length (Variables|Default|GetConsumableQuantityEquiped)) 0) ; Equip if they are the first Consumable
      (Default|SetEquip (LocalVariables|GetConsumable) true)
      (Consumables|EquipConsumables (Utilities|Struct|MakeStruct_ConsumableQuantity (LocalVariables|GetConsumable) (LocalVariables|GetAmount))))
    (else
      (Variables|Default|SetNewItemAmount 0)
      (return false))))

(fn RemoveConsumables
  (params (AmountToRemove :type Integer) (Struct_ConsumableQuantity :type Struct%20Consumable%20Quantity%20Structure%20%28by%20ref%29))
  (bind (_consumable _quantity) (Utilities|Struct|BreakStruct_ConsumableQuantity Struct_ConsumableQuantity))
  ;[0 0 0] Remove Quantity from Inventory
  (if (> _quantity 0)
    (for (_array_element _array_index) (Variables|Default|GetConsumableQuantity) ; FindItemToRemove
      (if (== (.Consumable (Utilities|Struct|BreakStruct_ConsumableQuantity _array_element)) _consumable)
        (Consumables|RemoveAmountConsumables _array_index (.Consumable (Utilities|Struct|BreakStruct_ConsumableQuantity _array_element)) AmountToRemove) ; Subtrack Quanty
        (Default|CallEEquiped self)
        (return true)))))

(fn ComsumableSelected
  (params (ItemAddIndex :type Integer))
  (bind _consumablequantityequiped (Variables|Default|GetConsumableQuantityEquiped))
  (bind _consumablequantityequiped_2 (Variables|Default|GetConsumableQuantityEquiped))
  (bind _returnvalue (Utilities|Array|LastIndex _consumablequantityequiped_2))
  (bind _output (Utilities|Array|Get(acopy) _consumablequantityequiped))
  (bind _output_2 (Utilities|Array|Get(acopy) _consumablequantityequiped_2 _returnvalue))
  ;[0 0 0] Switch Selected Consumable
  (Variables|Default|SetConsumableEquipedIndex (+ ItemAddIndex (Variables|Default|GetConsumableEquipedIndex)))
  (if (> (Variables|Default|GetConsumableEquipedIndex) (Utilities|Array|LastIndex (Variables|Default|GetConsumableQuantityEquiped)))
    ;[0 0 0] Set Selected Consumable
    ;;[0.3802 0.3802 0.3802] Set to first index
    (Utilities|IsValid (.Consumable (Utilities|Struct|BreakStruct_ConsumableQuantity _output)) ; Ensures a valid object is selected before setting.
      (:Is%20Valid
        (Variables|Default|SetConsumableEquipedIndex 0)
        (bind _output_get (Variables|Default|SetCurrentSelectedConsumable _output))
        (Consumables|MakeUIConsumable _output_get))
      (:Is%20Not%20Valid
        (Utilities|Array|RemoveIndex _consumablequantityequiped)
        (Default|CallEConsumableDeselect)))
    (else
      ;;[0.3802 0.3802 0.3802] Cycle though Array
      (if (< (Variables|Default|GetConsumableEquipedIndex) 0) ; Iterates through the equipped consumables to find the next valid item.\nSkips null/invalid entries and wraps around to first if needed.\nUpdates the HUD and sets the new selected item.
        (Utilities|IsValid (.Consumable (Utilities|Struct|BreakStruct_ConsumableQuantity _output_2))
          (:Is%20Valid
            (bind _output_get_2 (Variables|Default|SetConsumableEquipedIndex _returnvalue))
            (bind _output_get_3 (Variables|Default|SetCurrentSelectedConsumable _output_2))
            (Consumables|MakeUIConsumable _output_get_3))
          (:Is%20Not%20Valid
            (Utilities|Array|RemoveIndex (Variables|Default|GetConsumableQuantityEquiped) _output_get_2)
            (Default|CallEConsumableDeselect)))
        (else
          ;;[0.3802 0.3802 0.3802] SetLastArray
          (Utilities|IsValid (.Consumable (Utilities|Struct|BreakStruct_ConsumableQuantity (Utilities|Array|Get(acopy) (Variables|Default|GetConsumableQuantityEquiped) (Variables|Default|GetConsumableEquipedIndex)))) ; After removing a consumable, this function selects the last valid item in the list.\nEnsures the UI doesn't reference a removed/invalid object.
            (:Is%20Valid
              (bind _output_get_4 (Variables|Default|SetCurrentSelectedConsumable (Utilities|Array|Get(acopy) (Variables|Default|GetConsumableQuantityEquiped) (Variables|Default|GetConsumableEquipedIndex))))
              (Consumables|MakeUIConsumable _output_get_4))
            (:Is%20Not%20Valid
              (Utilities|Array|RemoveIndex (Variables|Default|GetConsumableQuantityEquiped) (Variables|Default|GetConsumableEquipedIndex))
              (Default|CallEConsumableDeselect)))))))
  (Default|CallEEquiped self) ; UpdateInventory
)

(fn RemoveAmountConsumables
  (params (Index :type Integer) (ConsumableToRemove :type BPD%20Consumable%20Data%20Object%20Reference) (Amount%20to%20Remove :type Integer))
  (bind _consumablequantity (Variables|Default|GetConsumableQuantity))
  ;[0 0 0] Update Inventory Stack After Use
  (LocalVariables|SetIndexAmountRemove Index)
  (Variables|Default|SetNewItemAmount (- (.Quantity (Utilities|Struct|BreakStruct_ConsumableQuantity (Utilities|Array|Get(acopy) (Variables|Default|GetConsumableQuantityEquiped) Index))) Amount%20to%20Remove))
  (Utilities|IsValid ConsumableToRemove
    (:Is%20Valid
      (Utilities|Array|SetArrayElem (Variables|Default|GetConsumableQuantityEquiped) (LocalVariables|GetIndexAmountRemove) (Utilities|Struct|MakeStruct_ConsumableQuantity ConsumableToRemove (Variables|Default|GetNewItemAmount))) ; Set New Quantity
      (for (_array_element _array_index) _consumablequantity ; Check if equiped
        (if (== ConsumableToRemove (.Consumable (Utilities|Struct|BreakStruct_ConsumableQuantity _array_element)))
          (Utilities|Array|SetArrayElem _consumablequantity _array_index (Utilities|Struct|MakeStruct_ConsumableQuantity ConsumableToRemove (Variables|Default|GetNewItemAmount))) ; Set New Quantity
        ))
      (Consumables|MakeUIConsumable (Utilities|Array|Get(acopy) (Variables|Default|GetConsumableQuantityEquiped) (LocalVariables|GetIndexAmountRemove))) ; Swich UI in player hud
      (Variables|Default|SetCurrentSelectedConsumable (Utilities|Array|Get(acopy) (Variables|Default|GetConsumableQuantityEquiped) (LocalVariables|GetIndexAmountRemove)))
      (Default|CallEEquiped self))))

(fn AddWeapon
  (params (Weapon%20Pickup :type BPD%20Weapon%20Data%20Object%20Reference))
  ;[1 1 1] Add Weapon To Inventory
  (Variables|Default|SetWeapon%20Pickup Weapon%20Pickup)
  (for _array_element (Variables|Default|GetWeaponsInventory) ; Check if New
    (if (== (Variables|Default|GetWeapon%20Pickup) _array_element)
      (LocalVariables|SetHasAlready true)))
  (if (not (LocalVariables|GetHasAlready))
    (bind _returnvalue (Utilities|Array|Add (Variables|Default|GetWeaponsInventory) (Variables|Default|GetWeapon%20Pickup))) ; Add toInventory
    (if (not (>= _returnvalue 1)) ; If first Add to Equiped
      (Utilities|Array|Add (Variables|Default|GetWeaponsEquiped) (Variables|Default|GetWeapon%20Pickup))
      (Default|SetEquip (Variables|Default|GetWeapon%20Pickup) true)
      (Default|CallESwitchWeapon (Variables|Default|GetWeapon%20Pickup)))))

(fn ItemAdded
  (params (ItemData :type BPD%20Item%20Data%20Object%20Reference) (Amount :type Integer))
  ;[0 0 0] Triggered when a new item is added to the inventory.
  (Utilities|IsValid ItemData
    (:Is%20Valid
      (Default|SetEquip ItemData false) ; Marks item as Not equipped upon pickup
      (switch Utilities|FlowControl|Switch|SwitchonE_ItemType (Variables|/Game/SoulsLlike/Light/DataAssets/BPD_ItemData.BPD_ItemData_C|GetItemType ItemData) ; Checks items type (Armor, Weapon, Consumable, Shield).\nEach type is cast and added to its corresponding inventory function.
        (:NewEnumerator1
          (Armor|AddArmor (.AsBPD%20Armor%20Data (Utilities|Casting|CastToBPD_ArmorData ItemData))))
        (:NewEnumerator2
          (Consumables|AddConsumables (.AsBPD%20Consumable%20Data (Utilities|Casting|CastToBPD_ConsumableData ItemData)) Amount))
        (:NewEnumerator3
          (Weapons|AddWeapon (.AsBPD%20Weapon%20Data (Utilities|Casting|CastToBPD_WeaponData ItemData))))
        (:NewEnumerator4
          (Shield|AddShield (.AsBPD%20Shield%20Data (Utilities|Casting|CastToBPD_ShieldData ItemData))))))))

(fn EquipWeapon
  (params (Equip%20Weapon :type BPD%20Weapon%20Data%20Object%20Reference))
  (Utilities|IsValid Equip%20Weapon
    (:Is%20Valid
      (bind _returnvalue (Utilities|Array|Add (Variables|Default|GetWeaponsEquiped) Equip%20Weapon))
      (Variables|Default|SetWeaponIndex _returnvalue)
      (Math|Integer|IncrementInt (Variables|Default|GetWeaponEquipedIndex)
        (:%20%20
          (Default|CallEEquiped self)
          (Default|CallESwitchWeapon Equip%20Weapon))))))

(fn UnequipWeapons
  (params (UnequipWeapons :type BPD%20Weapon%20Data%20Object%20Reference) (CanFillter :type Boolean))
  (bind _weaponsequiped (Variables|Default|GetWeaponsEquiped))
  ;[0 0 0] Unequip Weapons
  (Utilities|Array|RemoveItem _weaponsequiped UnequipWeapons) ; Remove From Equiped Array
  (Math|Integer|DecrementInt (Variables|Default|GetWeaponEquipedIndex)
    (:%20%20
      (Default|CallEFillterStore)
      (Default|CallEUpdateInventory self)
      (for _array_element _weaponsequiped ; Switch Weapon
        (if (== _array_element UnequipWeapons)
          (Default|SetEquip UnequipWeapons true)
          (Weapons|WeaponSeleced (Variables|Default|GetWeaponEquipedIndex))))
      (Default|CallEEquiped self)
      (Weapons|WeaponSeleced))))

(fn CanUnequipWeapon
  (return (> (Variables|Default|GetWeaponEquipedIndex) 1)))

(fn CanEquipWeapon
  (return (<= (Variables|Default|GetWeaponEquipedIndex) (Variables|Default|GetMaxWeapons))))

(fn AddArmor
  (params (ArmorInventory :type BPD%20Armor%20Data%20Object%20Reference))
  ;[0 0 0] Adds new armor item to the player’s inventory.
  (LocalVariables|SetArmorData ArmorInventory)
  (for _array_element (Variables|Default|GetArmorInventory)
    (for _array_element_2 (Variables|Default|GetArmorCharmsInventory) ; Checks if item already exists in any armor slot.
      (if (Math|Boolean|ORBoolean (== _array_element (LocalVariables|GetArmorData)) (== _array_element (Variables|Default|GetArmorChestInventory)) (== _array_element (Variables|Default|GetArmorHelmetInventory)) (== _array_element (Variables|Default|GetArmorLegsInventory)) (== _array_element _array_element_2)) ; Checks across all armor slots to see if item is already stored
        (LocalVariables|SetHasAlready true))))
  (if (not (LocalVariables|GetHasAlready))
    (Utilities|Array|Add (Variables|Default|GetArmorInventory) (LocalVariables|GetArmorData)) ; Adds To Armor Array
    (Default|CallEEquiped self)))

(fn EquipHelmet
  (params (ArmorInventory :type BPD%20Armor%20Data%20Object%20Reference))
  ;[0 0 0] Equips the selected Helmet armor from inventory.
  (if (Utilities|Select :Index (.Aromor (Utilities|Struct|BreakStruct_Armor (Variables|/Game/SoulsLlike/Light/DataAssets/BPD_ArmorData.BPD_ArmorData_C|GetAromor ArmorInventory))) :NewEnumerator0 false :NewEnumerator1 true :NewEnumerator2 false :NewEnumerator3 false :NewEnumerator4 false)
    (Variables|Default|SetArmorHelmetInventory ArmorInventory)
    (Default|CallEEquiped self)))

(fn EquipChest
  (params (ArmorInventory :type BPD%20Armor%20Data%20Object%20Reference))
  ;[0 0 0] Equips the selected Chest armor from inventory.
  (if (Utilities|Select :Index (.Aromor (Utilities|Struct|BreakStruct_Armor (Variables|/Game/SoulsLlike/Light/DataAssets/BPD_ArmorData.BPD_ArmorData_C|GetAromor ArmorInventory))) :NewEnumerator0 false :NewEnumerator1 false :NewEnumerator2 true :NewEnumerator3 false :NewEnumerator4 false)
    (Variables|Default|SetArmorChestInventory ArmorInventory)
    (Default|CallEEquiped self)))

(fn EquipLegs
  (params (ArmorInventory :type BPD%20Armor%20Data%20Object%20Reference))
  ;[0 0 0] Equips the selected leg armor from inventory.
  (if (Utilities|Select :Index (.Aromor (Utilities|Struct|BreakStruct_Armor (Variables|/Game/SoulsLlike/Light/DataAssets/BPD_ArmorData.BPD_ArmorData_C|GetAromor ArmorInventory))) :NewEnumerator0 false :NewEnumerator1 false :NewEnumerator2 false :NewEnumerator3 true :NewEnumerator4 false)
    (Variables|Default|SetArmorLegsInventory ArmorInventory)
    (Default|CallEEquiped self)))

(fn EquipCharms
  (params (ArmorInventory :type BPD%20Armor%20Data%20Object%20Reference))
  ;[0 0 0] Equips the selected Charm armor from inventory.
  (if (Utilities|Select :Index (.Aromor (Utilities|Struct|BreakStruct_Armor (Variables|/Game/SoulsLlike/Light/DataAssets/BPD_ArmorData.BPD_ArmorData_C|GetAromor ArmorInventory))) :NewEnumerator0 false :NewEnumerator1 false :NewEnumerator2 false :NewEnumerator3 false :NewEnumerator4 true)
    (Utilities|Array|Add (Variables|Default|GetArmorCharmsInventory) ArmorInventory) ; Can Add 2 Charms
    (Math|Integer|IncrementInt (Variables|Default|GetCharmEquipedIndex)
      (:%20%20
        (Default|CallEEquiped self)))))

(fn UnequipLegs
  (params (Target :type BPD%20Armor%20Data%20Object%20Reference))
  (if (and (== Target (Variables|Default|GetArmorLegsInventory)) (Utilities|Select :Index (.Aromor (Utilities|Struct|BreakStruct_Armor (Variables|/Game/SoulsLlike/Light/DataAssets/BPD_ArmorData.BPD_ArmorData_C|GetAromor Target))) :NewEnumerator0 false :NewEnumerator1 false :NewEnumerator2 false :NewEnumerator3 true :NewEnumerator4 false))
    (Variables|Default|SetArmorLegsInventory 0)
    (Default|CallEEquiped self)))

(fn UnequipChest
  (params (Target :type BPD%20Armor%20Data%20Object%20Reference))
  (if (and (== Target (Variables|Default|GetArmorChestInventory)) (Utilities|Select :Index (.Aromor (Utilities|Struct|BreakStruct_Armor (Variables|/Game/SoulsLlike/Light/DataAssets/BPD_ArmorData.BPD_ArmorData_C|GetAromor Target))) :NewEnumerator0 false :NewEnumerator1 false :NewEnumerator2 true :NewEnumerator3 false :NewEnumerator4 false))
    (Variables|Default|SetArmorChestInventory 0)
    (Default|CallEEquiped self)))

(fn UnequipHelme
  (params (Target :type BPD%20Armor%20Data%20Object%20Reference))
  (if (and (== Target (Variables|Default|GetArmorHelmetInventory)) (Utilities|Select :Index (.Aromor (Utilities|Struct|BreakStruct_Armor (Variables|/Game/SoulsLlike/Light/DataAssets/BPD_ArmorData.BPD_ArmorData_C|GetAromor Target))) :NewEnumerator0 false :NewEnumerator1 true :NewEnumerator2 false :NewEnumerator3 false :NewEnumerator4 false))
    (Variables|Default|SetArmorHelmetInventory 0)
    (Default|CallEEquiped self)))

(fn UnequipCharms
  (params (Target :type BPD%20Armor%20Data%20Object%20Reference))
  (bind _armorcharmsinventory (Variables|Default|GetArmorCharmsInventory))
  (if (Utilities|Select :Index (.Aromor (Utilities|Struct|BreakStruct_Armor (Variables|/Game/SoulsLlike/Light/DataAssets/BPD_ArmorData.BPD_ArmorData_C|GetAromor Target))) :NewEnumerator0 false :NewEnumerator1 false :NewEnumerator2 false :NewEnumerator3 false :NewEnumerator4 true)
    (Utilities|Array|RemoveItem _armorcharmsinventory Target)
    (Math|Integer|DecrementInt (Variables|Default|GetCharmEquipedIndex)
      (:%20%20
        (Default|CallEFillterStore)
        (Default|CallEUpdateInventory self)
        (for _array_element _armorcharmsinventory
          (if (== Target _array_element)
            (Default|SetEquip _array_element true)))
        (Default|CallEEquiped self)))))

(fn EquipConsumables
  (params (DataAssets :type Struct%20Consumable%20Quantity%20Structure%20%28by%20ref%29))
  ;[0 0 0] Equip Consumables and add to equiped menu
  (LocalVariables|SetnewConsumable DataAssets)
  (Utilities|IsValid (.Consumable (Utilities|Struct|BreakStruct_ConsumableQuantity DataAssets))
    (:Is%20Valid
      (if (LocalVariables|GetIsNew?) ; Is Item New
        (Variables|Default|SetNewItemAmount 0)
        (bind _returnvalue (Utilities|Array|Add (Variables|Default|GetConsumableQuantityEquiped) (LocalVariables|GetnewConsumable))) ; Add to the equiped Array
        (bind _output_get (Variables|Default|SetConsumableEquipedIndex _returnvalue))
        (Consumables|ComsumableSelected _output_get)
        (LocalVariables|SetIsNew? false)
        (Default|CallESwitchComsumable (.Icon (Utilities|Struct|BreakStruct_ItemHeader (Variables|/Game/SoulsLlike/Light/DataAssets/BPD_ItemData.BPD_ItemData_C|GetItemInfo (.Consumable (Utilities|Struct|BreakStruct_ConsumableQuantity (LocalVariables|GetnewConsumable)))))) (.Name (Utilities|Struct|BreakStruct_ItemHeader (Variables|/Game/SoulsLlike/Light/DataAssets/BPD_ItemData.BPD_ItemData_C|GetItemInfo (.Consumable (Utilities|Struct|BreakStruct_ConsumableQuantity (LocalVariables|GetnewConsumable)))))) (.Quantity (Utilities|Struct|BreakStruct_ConsumableQuantity (LocalVariables|GetnewConsumable)))) ; Switch to  new Equiped
        (Default|CallEEquiped self)
        (return true)
        (else
          (Variables|Default|SetNewItemAmount 0)
          (return false))))))

(fn UnequipConsumables
  (params (Struct_ConsumableQuantity :type Struct%20Consumable%20Quantity%20Structure%20%28by%20ref%29))
  ;[0 0 0] Remove From Equiped menu array
  (Utilities|IsValid (.Consumable (Utilities|Struct|BreakStruct_ConsumableQuantity Struct_ConsumableQuantity))
    (:Is%20Valid
      (Utilities|Array|RemoveItem (Variables|Default|GetConsumableQuantityEquiped) Struct_ConsumableQuantity) ; Remove From Equiped Array
      (Math|Integer|DecrementInt (Variables|Default|GetConsumableEquipedIndex)
        (:%20%20
          (Default|CallEFillterStore)
          (Default|CallEUpdateInventory self)
          (for _array_element (Variables|Default|GetConsumableQuantityEquiped)
            (if (== (.Consumable (Utilities|Struct|BreakStruct_ConsumableQuantity _array_element)) (.Consumable (Utilities|Struct|BreakStruct_ConsumableQuantity Struct_ConsumableQuantity)))
              (Default|SetEquip (.Consumable (Utilities|Struct|BreakStruct_ConsumableQuantity _array_element)) false) ; UnEquip
              (Consumables|ComsumableSelected (Variables|Default|GetConsumableEquiped)) ; Switch in HUD
            ))
          (Consumables|ComsumableSelected)
          (Default|CallEEquiped self))))))

(fn MakeUIConsumable
  (params (Struct_ConsumableQuantity :type Struct%20Consumable%20Quantity%20Structure%20%28by%20ref%29))
  (bind (_consumable _quantity) (Utilities|Struct|BreakStruct_ConsumableQuantity Struct_ConsumableQuantity))
  (bind _iteminfo (Variables|/Game/SoulsLlike/Light/DataAssets/BPD_ItemData.BPD_ItemData_C|GetItemInfo _consumable))
  (bind (_icon _name) (Utilities|Struct|BreakStruct_ItemHeader _iteminfo))
  ;[0 0 0] Switch UI HUD Displayed Consumable
  (Utilities|IsValid _consumable
    (:Is%20Valid
      (Default|CallESwitchComsumable _icon _name _quantity))))

(fn AddShield
  (params (Shield :type BPD%20Shield%20Data%20Object%20Reference))
  ;[0 0 0] Add Shield too inventory
  (for _array_element (Variables|Default|GetShieldInventory)
    (if (or (== (Variables|Default|GetShieldInventoryEquiped) _array_element) (== Shield _array_element))
      (LocalVariables|SetHasAlready true)))
  (if (not (LocalVariables|GetHasAlready))
    (Utilities|Array|Add (Variables|Default|GetShieldInventory) Shield)
    (Default|CallEEquiped self)))

(fn EquipShield
  (params (Shield :type BPD%20Shield%20Data%20Object%20Reference))
  ;[0 0 0] Equip Selected Shield
  (Variables|Default|SetShieldInventoryEquiped Shield)
  (Default|CallEEquiped self))

(fn UnequipShield
  (params (Shield :type BPD%20Shield%20Data%20Object%20Reference))
  (if (== Shield (Variables|Default|GetShieldInventoryEquiped))
    (Variables|Default|SetShieldInventoryEquiped 0)
    (Default|CallEEquiped self)))