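; Player stats component for a Souls-like game, tracking health and stamina against PlayerInfo maximums and notifying UI through event calls.
; Health changes trigger player death at zero, otherwise a hit reaction that blocks attacking and plays montages under a Busy gameplay tag.
; Stamina changes return success or failure, with timers handling delayed, looping regeneration after use or depletion.
; HitCondisions checks cooldown, rolling and player state, but its branches perform no action.
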(event Custom|Reset
  (bind _player (Class|BPIPlayer|GetPlayer(Message) (Components|GetOwner)))
  (Variables|Default|SetPlayer _player)
  (bind _output_get (Variables|Default|SetCurrentHealth (.MaxHealth (Utilities|Struct|BreakStruct_PlayerStats (Variables|/Game/SoulsLlike/Light/BluePrints/Player/BP_BaseSoulsChap.BP_BaseSoulsChap_C|GetPlayerInfo (Variables|Default|GetPlayer))))))
  (bind _output_get_2 (Variables|Default|SetCurrentStanima (.MaxStanima (Utilities|Struct|BreakStruct_PlayerStats (Variables|/Game/SoulsLlike/Light/BluePrints/Player/BP_BaseSoulsChap.BP_BaseSoulsChap_C|GetPlayerInfo (Variables|Default|GetPlayer))))))
  (Default|CallEStanimaUpdataUI _output_get_2)
  (Default|CallEHealthUpdataUI _output_get))

(event EventBeginPlay
  (bind _player (Class|BPIPlayer|GetPlayer(Message) (Components|GetOwner)))
  (Variables|Default|SetPlayer _player)
  (bind _output_get (Variables|Default|SetCurrentHealth (.MaxHealth (Utilities|Struct|BreakStruct_PlayerStats (Variables|/Game/SoulsLlike/Light/BluePrints/Player/BP_BaseSoulsChap.BP_BaseSoulsChap_C|GetPlayerInfo (Variables|Default|GetPlayer))))))
  (bind _output_get_2 (Variables|Default|SetCurrentStanima (.MaxStanima (Utilities|Struct|BreakStruct_PlayerStats (Variables|/Game/SoulsLlike/Light/BluePrints/Player/BP_BaseSoulsChap.BP_BaseSoulsChap_C|GetPlayerInfo (Variables|Default|GetPlayer))))))
  (Default|CallEStanimaUpdataUI _output_get_2)
  (Default|CallEHealthUpdataUI _output_get))

(event Custom|CooldownHealth
  ;[0.15 0.15 0.15 0.5] The player gets stund
  (Variables|Default|SetCanUpdateHealthCoolDown true))

(event Custom|TakeHit
  (bind _player (Variables|Default|GetPlayer))
  (bind _player_2 (Variables|Default|GetPlayer))
  (bind _playertagsactions (Variables|/Game/SoulsLlike/Light/BluePrints/Player/BP_BaseSoulsChap.BP_BaseSoulsChap_C|GetPlayerTagsActions _player))
  ;[0.15 0.15 0.15 0.5] The player gets stund
  (Class|BPIWeapon|DoNotAttack(Message) (Variables|/Script/Engine.ChildActorComponent|GetChildActor (Variables|/Game/SoulsLlike/Light/BluePrints/Player/BP_BaseSoulsChap.BP_BaseSoulsChap_C|GetBP_BaseWeapon _player_2)))
  (Default|VisWeapon _player_2)
  (for _array_element (Variables|/Game/SoulsLlike/Light/BluePrints/Player/BP_BaseSoulsChap.BP_BaseSoulsChap_C|GetArrayOfSM (Variables|Default|GetPlayer))
    (Animation|Montage|PlayMontage _array_element "/Game/SoulsLlike/Heavy/Anims/Montages/AM_Hit.AM_Hit" 1.6
      (:then
        (GameplayTags|AddGameplayTag _playertagsactions "(TagName=\"CharacterActoins.Busy\")" :!class /Script/GameplayTags.BlueprintGameplayTagLibrary))
      (:OnCompleted
        (GameplayTags|RemoveGameplayTag _playertagsactions "(TagName=\"CharacterActoins.Busy\")" :!class /Script/GameplayTags.BlueprintGameplayTagLibrary)))))

(event EventHealthUpdata
  (params (Value :type Float%20%28double-precision%29))
  ;[0.15 0.15 0.15 0.5] The Current Health has changed
  (Utilities|Time|SetTimerbyEvent (EventDispatchers|CreateEvent :!event Custom|CooldownHealth) 1.0)
  (Variables|Default|SetCanUpdateHealthCoolDown false)
  (bind _player (Class|BPIPlayer|GetPlayer(Message) (Components|GetOwner)))
  (Variables|Default|SetPlayer _player)
  (CallFunction|HitCondisions)
  (Variables|Default|SetCurrentHealth (Math|Float|Clamp(Float) (+ Value (Variables|Default|GetCurrentHealth)) 0.0 (Utilities|Struct|BreakStruct_PlayerStats (Variables|/Game/SoulsLlike/Light/BluePrints/Player/BP_BaseSoulsChap.BP_BaseSoulsChap_C|GetPlayerInfo (Variables|Default|GetPlayer)))))
  (Default|CallEHealthUpdataUI (Variables|Default|GetCurrentHealth))
  (if (<= (Variables|Default|GetCurrentHealth) 0.0) ; HasHealthLeft
    (Default|PlayerDeath (Variables|/Game/SoulsLlike/Light/BluePrints/Player/BP_BaseSoulsChap.BP_BaseSoulsChap_C|GetBPC_Respawn (Variables|Default|GetPlayer)))
    (else
      (CallFunction|TakeHit))))

(fn HitCondisions
  (bind _player (Variables|Default|GetPlayer))
  (if (Variables|Default|GetCanUpdateHealthCoolDown)
    (if (not (Math|Boolean|ANDBoolean (Utilities|IsValid _player) (GameplayTags|HasTag (Variables|/Game/SoulsLlike/Light/BluePrints/Player/BP_BaseSoulsChap.BP_BaseSoulsChap_C|GetPlayerTagsActions _player) "(TagName=\"CharacterActoins.Busy.Rolling\")") (Utilities|Select :Index (Variables|/Game/SoulsLlike/Light/BluePrints/Player/BP_BaseSoulsChap.BP_BaseSoulsChap_C|GetPlayersState _player) :NewEnumerator0 false :NewEnumerator1 true :NewEnumerator2 true :NewEnumerator3 false :NewEnumerator4 false :NewEnumerator6 false :NewEnumerator7 false :NewEnumerator11 false :NewEnumerator13 true)))
      _)))

(fn FullStaminaRegeneration
  (bind _player (Variables|Default|GetPlayer))
  (bind _playerinfo (Variables|/Game/SoulsLlike/Light/BluePrints/Player/BP_BaseSoulsChap.BP_BaseSoulsChap_C|GetPlayerInfo _player))
  (bind _maxstanima (Utilities|Struct|BreakStruct_PlayerStats _playerinfo))
  (bind _output_get (Variables|Default|SetCurrentStanima (Math|Float|Clamp(Float) (+ (Variables|Default|GetCurrentStanima) (Variables|Default|GetRegenStanimaValue)) 0.0 _maxstanima)))
  (Default|CallEStanimaUpdataUI _output_get)
  (if (>= (Variables|Default|GetCurrentStanima) _maxstanima)
    (CallFunction|ClearTimer)))

(fn ClearTimer
  (Utilities|Time|ClearandInvalidateTimerbyHandle (Variables|Default|GetCoolDownHandle))
  (Utilities|Time|ClearandInvalidateTimerbyHandle (Variables|Default|GetStartRegenHandle))
  (Utilities|Time|ClearandInvalidateTimerbyHandle (Variables|Default|GetRegenStanimaCooldownHanle)))

(fn DecressStanima
  (params (Value :type Float%20%28double-precision%29))
  (bind _player (Class|BPIPlayer|GetPlayer(Message) (Components|GetOwner)))
  (Variables|Default|SetPlayer _player)
  (Variables|Default|SetCurrentStanima (Math|Float|Clamp(Float) (+ Value (Variables|Default|GetCurrentStanima)) 0.0 (Utilities|Struct|BreakStruct_PlayerStats (Variables|/Game/SoulsLlike/Light/BluePrints/Player/BP_BaseSoulsChap.BP_BaseSoulsChap_C|GetPlayerInfo (Variables|Default|GetPlayer))))) ; Set New current stanima
  (Default|CallEStanimaUpdataUI (Variables|Default|GetCurrentStanima)))

(fn RegenerateStanimaTimer
  (bind _returnvalue (Utilities|Time|SetTimerbyEvent (EventDispatchers|CreateEvent :!event RegenerateStanima) 0.2 true)) ; How often regen in a loop
  (Variables|Default|SetStartRegenHandle _returnvalue))

(fn NeedMoreStanima
  (Default|CallENeedMoreStanima)
  (bind _returnvalue (Utilities|Time|SetTimerbyEvent (EventDispatchers|CreateEvent :!event RegenerateStanimaTimer) 0.8)) ; Cool down till regen
  (Variables|Default|SetCoolDownHandle _returnvalue))

(fn RegenerateStanima
  (Variables|Default|SetCurrentStanima (Math|Float|Clamp(Float) (+ (Variables|Default|GetCurrentStanima) (Variables|Default|GetRegenStanimaValue)) 0.0 (Utilities|Struct|BreakStruct_PlayerStats (Variables|/Game/SoulsLlike/Light/BluePrints/Player/BP_BaseSoulsChap.BP_BaseSoulsChap_C|GetPlayerInfo (Variables|Default|GetPlayer)))))
  (Default|CallEStanimaUpdataUI (Variables|Default|GetCurrentStanima))
  (if (<= (Variables|Default|GetCurrentStanima) 0.0)
    (Utilities|Time|ClearandInvalidateTimerbyHandle (Variables|Default|GetStartRegenHandle))))

(fn RegenerateStanimaCooldownTimer
  (bind _returnvalue (Utilities|Time|SetTimerbyEvent (EventDispatchers|CreateEvent :!event RegenerateStanimaTimer) 1.2)) ; Regen cooldown
  (Variables|Default|SetRegenStanimaCooldownHanle _returnvalue))

(fn StanimaUpdata
  (params (Value :type Float%20%28double-precision%29))
  (CallFunction|ClearTimer)
  (if (> (+ Value (Variables|Default|GetCurrentStanima)) 0.0)
    (CallFunction|DecressStanima Value)
    (CallFunction|RegenerateStanimaCooldownTimer)
    (return true) ; Success enough stanima the use
    (else
      (CallFunction|NeedMoreStanima)
      (return false) ; Not enough stanima to use fail
    )))