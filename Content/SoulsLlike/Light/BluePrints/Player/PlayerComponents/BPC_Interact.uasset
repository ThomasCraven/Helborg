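; BPC_Interact is a player component that handles interaction with nearby objects such as pickups and bonfires.
; On interact input, a sphere trace at the capsule finds BPI_Interact actors and messages the one matching the stored overlapping actor.
; Bonfires trigger the player's rest state; other successes play force feedback, clear the popup and refresh prompts.
; Prompt refresh repeats the trace and opens pickup messages on every interactable hit.
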(event Custom|InteractionBreak
  ;[0 0 0] Player Interact Input → Trace for Pickup Object
  (Utilities|Array|ForEachLoopwithBreak (stale Input|EnhancedActionEvents|EnhancedInputActionIA_Interact _outhits)) ; enters at Break
)

(event Custom|UpdateInteractionPromptPopUp
  (bind _player (Variables|Default|GetPlayer))
  (bind _capsulecomponent (Variables|/Script/Engine.Character|GetCapsuleComponent _player))
  (bind _returnvalue (Transformation|GetSocketLocation _capsulecomponent "None"))
  ;[0 0 0] Runs when player enters an overlap zone. Validates the overlapped actor, performs a sphere trace, and stores the nearest valid interactable.
  (Utilities|IsValid _player
    (:Is%20Valid
      (bind (_outhits _returnvalue_2) (Collision|MultiSphereTraceByChannel _returnvalue _returnvalue (Variables|Default|GetRadiusOfInteract) "TraceTypeQuery1" false 0 "None"))
      (if _returnvalue_2
        (for _array_element _outhits
          (CallFunction|GetCorrectActor _array_element))))))

(event Custom|Overlapping
  (params (OverlapingActor :type Actor%20Object%20Reference))
  ;[0 0 0] Checks if the overlapping actor is valid, and sets up internal flags if interaction is possible.
  (Utilities|IsValid OverlapingActor
    (:Is%20Valid
      (Variables|Default|SetOverlaping%20Actor OverlapingActor))))

(event Input|EnhancedActionEvents|EnhancedInputActionIA_Interact
  (params (ActionValue :type Boolean) (ElapsedSeconds :type Float%20%28double-precision%29) (TriggeredSeconds :type Float%20%28double-precision%29) (InputAction :type Input%20Action%20Object%20Reference :default "/Game/SoulsLlike/Light/Inputs/InputAcsions/IA_Interact.IA_Interact"))
  (bind _player (Variables|Default|GetPlayer))
  (bind _capsulecomponent (Variables|/Script/Engine.Character|GetCapsuleComponent _player))
  (bind _returnvalue (Transformation|GetSocketLocation _capsulecomponent "None"))
  ;[0 0 0] Player Interact Input → Trace for Pickup Object
  (if (Default|CanMakeAcsoin _player) ; RightPlayerState
    (bind (_outhits _returnvalue_2) (Collision|MultiSphereTraceByChannel _returnvalue _returnvalue (Variables|Default|GetRadiusOfInteract) "TraceTypeQuery1" false 0 "None")) ; Gets the center point for the trace
    (if _returnvalue_2
      (bind _array_element (Utilities|Array|ForEachLoopwithBreak _outhits) ; Handles the actual Interactoin logic after a valid actor is found. So picks up once
        (:LoopBody
          (CallFunction|InterctwithHitActors _array_element))))))

(fn InteractEffect
  (ForceFeedback|SpawnForceFeedbackatLocation "/Game/SoulsLlike/Light/Inputs/Feedback/FF_VeryQuick.FF_VeryQuick" (Transformation|GetSocketLocation (Variables|/Script/Engine.Actor|GetRootComponent (Variables|Default|GetPlayer)) "None") "0, 0, 0" false 1.0 0.0 0))

(fn InteractwithBonfireEffect
  (params (InputPin :type Actor%20Object%20Reference))
  (bind _player (Variables|Default|GetPlayer))
  (Class|BPIBonFire|Rest(Message) InputPin)
  (Variables|/Game/SoulsLlike/Light/BluePrints/Player/BP_BaseSoulsChap.BP_BaseSoulsChap_C|SetBonfire _player InputPin)
  (Default|RestatBonFire _player)
  (CallFunction|InteractionBreak))

(fn IsInteractable
  (params (HitActor :type Object%20Object%20Reference))
  (return (Utilities|DoesObjectImplementInterface HitActor "/Game/SoulsLlike/Light/BluePrints/Interfaces/BPI_Interact.BPI_Interact_C")))

(fn InterctwithHitActors
  (params (Hit :type Hit%20Result%20Structure%20%28by%20ref%29))
  (bind _hitactor (Collision|BreakHitResult Hit))
  (if (Math|Boolean|ANDBoolean (Default|CanMakeAcsoin (Variables|Default|GetPlayer)) (CallFunction|IsInteractable _hitactor) (== _hitactor (Variables|Default|GetOverlaping%20Actor)))
    (CallFunction|InteractionBreak)
    (bind _success (Class|BPIInteract|Interact(Message) (Variables|Default|GetOverlaping%20Actor) true (Variables|Default|GetPlayer))) ; Interact With hit actor
    (if _success
      (if (Utilities|DoesObjectImplementInterface _hitactor "/Game/SoulsLlike/Light/BluePrints/Interfaces/BPI_BonFire.BPI_BonFire_C") ; If Bonfire
        (CallFunction|InteractwithBonfireEffect _hitactor)
        (else
          (CallFunction|InteractEffect)
          (Class|BPIPlayer|LeavePopUp(Message) (Variables|Default|GetPlayer))
          (CallFunction|UpdateInteractionPromptPopUp))))))

(fn GetCorrectActor
  (params (Hit :type Hit%20Result%20Structure%20%28by%20ref%29))
  (bind _hitactor (Collision|BreakHitResult Hit))
  (bind _player (Variables|Default|GetPlayer))
  (if (Utilities|DoesObjectImplementInterface _hitactor "/Game/SoulsLlike/Light/BluePrints/Interfaces/BPI_Interact.BPI_Interact_C") ; Is Intractable
    (Class|BPIInteract|OpenPickup(Message) _hitactor _player (Variables|/Script/Engine.Character|GetCapsuleComponent _player)) ; PopUpOnScreenThe conrectActor
  ))

(fn Initialise
  (params (Player :type BP%20Base%20Souls%20Chap%20Object%20Reference))
  (Variables|Default|SetPlayer Player))