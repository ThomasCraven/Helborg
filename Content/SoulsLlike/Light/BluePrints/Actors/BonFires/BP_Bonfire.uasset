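; Souls-like bonfire actor that the player first lights, then rests at, with popup prompts that switch on its active state.
; Box overlaps with player-interface actors show or clear the prompt through BPCPopUpUI.
; Interact marks resting, broadcasts bonfire state and fades in looping audio; first lighting adds burst VFX, force feedback and a timer for a delayed event.
; EndRest clears resting, restores the popup and fades out the sound.
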(event OnComponentBeginOverlap(Box)
  (params (OverlappedComponent :type Primitive%20Component%20Object%20Reference) (OtherActor :type Actor%20Object%20Reference) (OtherComp :type Primitive%20Component%20Object%20Reference) (OtherBodyIndex :type Integer) (bFromSweep :type Boolean) (SweepResult :type Hit%20Result%20Structure%20%28by%20ref%29))
  (if (and (Utilities|DoesObjectImplementInterface OtherActor "/Game/SoulsLlike/Light/BluePrints/Interfaces/BPI_Player.BPI_Player_C") (not (Variables|Default|GetIsResting)))
    (Variables|Default|SetPlayer OtherActor)
    (Variables|Default|SetOther%20Comp OtherComp)
    (if (Variables|Default|GetIsActive?)
      (Default|PopUp (Variables|Default|GetBPC_PopUpUI) (Variables|Default|GetRestAt) (Variables|Default|GetPlayer) 0 "NewEnumerator2" 0 (Variables|Default|GetOther%20Comp) 0 self)
      (else
        (Default|PopUp (Variables|Default|GetBPC_PopUpUI) (Variables|Default|GetLight%20Bon) (Variables|Default|GetPlayer) 0 "NewEnumerator6" 0 (Variables|Default|GetOther%20Comp) 0 self)))
    (Variables|Default|SetOther%20Comp 0)))

(event OnComponentEndOverlap(Box)
  (params (OverlappedComponent :type Primitive%20Component%20Object%20Reference) (OtherActor :type Actor%20Object%20Reference) (OtherComp :type Primitive%20Component%20Object%20Reference) (OtherBodyIndex :type Integer))
  (Default|LeavePopUp (Variables|Default|GetBPC_PopUpUI) OtherActor OtherComp))

(event Custom|LiteFire
  (Niagara|SpawnSystemAttached "/Game/SoulsLlike/Heavy/Systems/NS_Fire.NS_Fire" (Variables|Default|GetScene) "None" "0, 0, 0" "0, 0, 0" "KeepRelativeOffset" false))

(event EventOpenPickup
  (params (player :type BP%20Base%20Souls%20Chap%20Object%20Reference) (Component :type Primitive%20Component%20Object%20Reference))
  (Variables|Default|SetPlayer player)
  (Variables|Default|SetOther%20Comp Component)
  (if (Variables|Default|GetIsActive?)
    (Default|PopUp (Variables|Default|GetBPC_PopUpUI) (Variables|Default|GetRestAt) (Variables|Default|GetPlayer) 0 "NewEnumerator2" 0 (Variables|Default|GetOther%20Comp) 0 self)
    (else
      (Default|PopUp (Variables|Default|GetBPC_PopUpUI) (Variables|Default|GetLight%20Bon) (Variables|Default|GetPlayer) 0 "NewEnumerator6" 0 (Variables|Default|GetOther%20Comp) 0 self)))
  (Variables|Default|SetOther%20Comp 0))

(event EventEndRest
  (bind _firesound (Variables|Default|GetFireSound))
  (Variables|Default|SetIsResting false)
  (Class|BPIPlayer|Popup(Message) (Variables|Default|GetPlayer) (Variables|Default|GetLight%20Bon) 0 "NewEnumerator2")
  (Utilities|IsValid _firesound
    (:Is%20Valid
      (Audio|Components|Audio|FadeOut _firesound 2.0 0.0 "Linear" :!class /Script/Engine.AudioComponent))))

(fn ConstructionScript)

(fn Interact
  (params (HasIntracted? :type Boolean) (Player :type BP%20Base%20Souls%20Chap%20Object%20Reference))
  (Variables|Default|SetIsResting true)
  (Class|BPIPlayer|LeavePopUp(Message) (Variables|Default|GetPlayer))
  (if (Variables|Default|GetIsActive?)
    (Default|CallEBonFireActive false self)
    (Audio|PlaySound2D "/Game/SoulsLlike/Light/Sound/Effects/SW_Fire_Ward_002.SW_Fire_Ward_002" 1.0 1.0 0.0 0 0)
    (bind _returnvalue (Audio|CreateSound2D "/Game/SoulsLlike/Light/Sound/Effects/SW_Lava_Enchantment_Loop_001.SW_Lava_Enchantment_Loop_001" 1.0 1.0 0.0 0))
    (bind _output_get (Variables|Default|SetFireSound _returnvalue))
    (Audio|Components|Audio|FadeIn _output_get 0.5 1.0 0.0 "Linear" :!class /Script/Engine.AudioComponent)
    (return self true)
    (else
      (Niagara|SpawnSystematLocation "/Game/SoulsLlike/Heavy/Systems/NS_Boom.NS_Boom" (Transformation|GetSocketLocation (Variables|Default|Gete) "None"))
      (Variables|Default|SetIsActive? true)
      (Default|CallEBonFireActive (Variables|Default|GetIsActive?) self)
      (Audio|PlaySound2D "/Game/SoulsLlike/Light/Sound/Effects/Warm_Buff_001.Warm_Buff_001" 1.0 1.0 0.0 0 0)
      (bind _returnvalue_2 (Audio|CreateSound2D "/Game/SoulsLlike/Light/Sound/Effects/SW_Lava_Enchantment_Loop_001.SW_Lava_Enchantment_Loop_001" 1.0 1.0 0.0 0))
      (bind _output_get_2 (Variables|Default|SetFireSound _returnvalue_2))
      (Audio|Components|Audio|FadeIn _output_get_2 0.5 1.0 0.0 "Linear" :!class /Script/Engine.AudioComponent)
      (ForceFeedback|SpawnForceFeedbackatLocation "/Game/SoulsLlike/Light/Inputs/Feedback/FF_Quick.FF_Quick" (Transformation|GetActorLocation (Game|GetPlayerCharacter 0)) "0, 0, 0" false 1.0 0.0 0)
      (Utilities|Time|SetTimerbyEvent (EventDispatchers|CreateEvent :!event Custom|LiteFire) 1.0)
      (return self true))))