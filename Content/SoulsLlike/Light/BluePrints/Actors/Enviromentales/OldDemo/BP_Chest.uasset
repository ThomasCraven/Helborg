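; BP_Chest is an interactable chest that opens once and spawns a pickup for the player.
; Box overlap shows or hides a prompt through BPI_Player and stores the player reference.
; On interaction it clears the prompt, spawns the configured class with an amount, plays a sound and runs a timeline.
; The timeline rotates the lid by lerping its roll from the actor's starting rotation to OpenXPosition.
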(event OnComponentBeginOverlap(Box)
  (params (OverlappedComponent :type Primitive%20Component%20Object%20Reference) (OtherActor :type Actor%20Object%20Reference) (OtherComp :type Primitive%20Component%20Object%20Reference) (OtherBodyIndex :type Integer) (bFromSweep :type Boolean) (SweepResult :type Hit%20Result%20Structure%20%28by%20ref%29))
  (if (and (Utilities|DoesObjectImplementInterface OtherActor "/Game/SoulsLlike/Light/BluePrints/Interfaces/BPI_Player.BPI_Player_C") (not (Variables|Default|GetOpen?)))
    (Class|BPIPlayer|Popup(Message) OtherActor (Variables|Default|GetIntract%20With) 0 "NewEnumerator0")
    (Variables|Default|SetPlayerRef OtherActor)))

(event OnComponentEndOverlap(Box)
  (params (OverlappedComponent :type Primitive%20Component%20Object%20Reference) (OtherActor :type Actor%20Object%20Reference) (OtherComp :type Primitive%20Component%20Object%20Reference) (OtherBodyIndex :type Integer))
  (if (Utilities|DoesObjectImplementInterface OtherActor "/Game/SoulsLlike/Light/BluePrints/Interfaces/BPI_Player.BPI_Player_C")
    (Class|BPIPlayer|LeavePopUp(Message) OtherActor)))

(event Custom|Intract_1_1
  (params (HasIntracted? :type Boolean))
  (if (and HasIntracted? (not (Variables|Default|GetOpen?)))
    (Class|BPIPlayer|LeavePopupNow(Message) (Variables|Default|GetPlayerRef))
    (Variables|Default|SetOpen? true)
    (CallFunction|SpawnPickUp)
    (Audio|PlaySoundatLocation "/Game/SoulsLlike/Light/Sound/Effects/SW_Dungeon_Door_Open_Wet_B.SW_Dungeon_Door_Open_Wet_B" (Transformation|GetSocketLocation (Variables|Default|GetPick%20Spawn%20location) "None") "0, 0, 0" 1.0 1.0 0.0 0 0 0 0)
    (bind _alpha (Timeline|OpenChest Play)
      (:Update
        (CallFunction|OpenLocation _alpha)))))

(event EventBeginPlay
  (Variables|Default|SetStartTransform (Transformation|GetActorTransform)))

(fn ConstructionScript)

(fn OpenLocation
  (params (Alpha :type Float%20%28single-precision%29))
  (bind _starttransform (Variables|Default|GetStartTransform))
  (Transformation|SetWorldRotation (Variables|Default|GetSM_Prop_Chest_04_Lid) (Math|Rotator|Lerp(Rotator) (.rotation (Variables|Default|GetStartTransform)) (Math|Rotator|MakeRotator (Variables|Default|GetOpen%28x%29Position) (.pitch (.rotation _starttransform)) (.yaw (.rotation _starttransform))) Alpha true) false false))

(fn SpawnPickUp
  (bind _class (Variables|Default|GetClass)
    (:then
      (bind _returnvalue (Game|SpawnActorfromClass _class (Math|Transform|MakeTransform (Transformation|GetSocketLocation (Variables|Default|GetPick%20Spawn%20location) "None") "0, 0, 0" "1.000000,1.000000,1.000000") "Undefined" "MultiplyWithRoot" 0 0))
      (Class|BPIInteract|AddAmount(Message) _returnvalue (Variables|Default|GetAmount)))
    (:else)))

(fn Interact
  (params (HasIntracted? :type Boolean) (Player :type BP%20Base%20Souls%20Chap%20Object%20Reference))
  (return 0 false))