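; BP_Button is an interactable button actor that relays an interaction to an array of linked targets.
; Its box overlap sends a popup prompt to actors implementing BPI_Player and clears it when they leave.
; The Intract_1_1 event, when flagged as interacted, calls InteractMessage on every entry in the Inract array.
; The separate Interact function is a stub that always reports failure.
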(event OnComponentBeginOverlap(Box)
  (params (OverlappedComponent :type Primitive%20Component%20Object%20Reference) (OtherActor :type Actor%20Object%20Reference) (OtherComp :type Primitive%20Component%20Object%20Reference) (OtherBodyIndex :type Integer) (bFromSweep :type Boolean) (SweepResult :type Hit%20Result%20Structure%20%28by%20ref%29))
  (if (Utilities|DoesObjectImplementInterface OtherActor "/Game/SoulsLlike/Light/BluePrints/Interfaces/BPI_Player.BPI_Player_C")
    (Class|BPIPlayer|Popup(Message) OtherActor (Variables|Default|GetIntract%20With) 0 "NewEnumerator0")
    (else
      (Class|BPIPlayer|LeavePopUp(Message) OtherActor))))

(event OnComponentEndOverlap(Box)
  (params (OverlappedComponent :type Primitive%20Component%20Object%20Reference) (OtherActor :type Actor%20Object%20Reference) (OtherComp :type Primitive%20Component%20Object%20Reference) (OtherBodyIndex :type Integer))
  (if (Utilities|DoesObjectImplementInterface OtherActor "/Game/SoulsLlike/Light/BluePrints/Interfaces/BPI_Player.BPI_Player_C")
    (Class|BPIPlayer|LeavePopUp(Message) OtherActor)))

(event Custom|Intract_1_1
  (params (HasIntracted? :type Boolean))
  (if HasIntracted?
    (for _array_element (Variables|Default|GetInract)
      (Class|BPIInteract|Interact(Message) _array_element true))))

(fn ConstructionScript)

(fn Interact
  (params (HasIntracted? :type Boolean) (Player :type BP%20Base%20Souls%20Chap%20Object%20Reference))
  (return 0 false))