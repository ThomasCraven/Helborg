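; BP_SpikeThing is a one-time interactable that swings two Left and Right parts open like a double door and spawns an actor.
; An overlap box shows an interaction popup through BPI_Player while it is closed.
; The first interaction plays a wet dungeon-door sound at both parts, spawns the configured class at the Arrow, and runs a timeline that lerps their yaw outward from the rotations cached at BeginPlay.
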(event OnComponentBeginOverlap(Box)
  (params (OverlappedComponent :type Primitive%20Component%20Object%20Reference) (OtherActor :type Actor%20Object%20Reference) (OtherComp :type Primitive%20Component%20Object%20Reference) (OtherBodyIndex :type Integer) (bFromSweep :type Boolean) (SweepResult :type Hit%20Result%20Structure%20%28by%20ref%29))
  (if (and (Utilities|DoesObjectImplementInterface OtherActor "/Game/SoulsLlike/Light/BluePrints/Interfaces/BPI_Player.BPI_Player_C") (not (Variables|Default|GetOpen?)))
    (Class|BPIPlayer|Popup(Message) OtherActor (Variables|Default|GetIntract%20With) 0 "NewEnumerator0")
    (else
      (Class|BPIPlayer|LeavePopUp(Message) OtherActor))))

(event OnComponentEndOverlap(Box)
  (params (OverlappedComponent :type Primitive%20Component%20Object%20Reference) (OtherActor :type Actor%20Object%20Reference) (OtherComp :type Primitive%20Component%20Object%20Reference) (OtherBodyIndex :type Integer))
  (if (Utilities|DoesObjectImplementInterface OtherActor "/Game/SoulsLlike/Light/BluePrints/Interfaces/BPI_Player.BPI_Player_C")
    (Class|BPIPlayer|LeavePopUp(Message) OtherActor)))

(event Custom|Intract_1_1
  (params (HasIntracted? :type Boolean))
  (bind _startleft (Variables|Default|GetStartLeft))
  (bind _startrighrt (Variables|Default|GetStartRighrt))
  (if (and HasIntracted? (not (Variables|Default|GetOpen?)))
    (Variables|Default|SetOpen? true)
    (Audio|PlaySoundatLocation "/Game/SoulsLlike/Light/Sound/Effects/SW_Dungeon_Door_Open_Wet_B.SW_Dungeon_Door_Open_Wet_B" (Transformation|GetSocketLocation (Variables|Default|GetLeft) "None") "0, 0, 0" 1.0 1.0 0.0 0 0 0 0)
    (Audio|PlaySoundatLocation "/Game/SoulsLlike/Light/Sound/Effects/SW_Dungeon_Door_Open_Wet_B.SW_Dungeon_Door_Open_Wet_B" (Transformation|GetSocketLocation (Variables|Default|GetRight) "None") "0, 0, 0" 1.0 1.0 0.0 0 0 0 0)
    (Game|SpawnActorfromClass (Variables|Default|GetClass) (Math|Transform|MakeTransform (Transformation|GetSocketLocation (Variables|Default|GetArrow) "None") "0, 0, 0" "1.000000,1.000000,1.000000") "Undefined" "MultiplyWithRoot" 0 0)
    (bind _alpha (Timeline|Timeline Play)
      (:Update
        (Transformation|SetRelativeRotation (Variables|Default|GetRight) (Math|Rotator|Lerp(Rotator) (.rotation (Variables|Default|GetStartRighrt)) (Math|Rotator|MakeRotator (.roll (.rotation _startrighrt)) (.pitch (.rotation _startrighrt)) -1.2e+02) _alpha true) false false)
        (Transformation|SetRelativeRotation (Variables|Default|GetLeft) (Math|Rotator|Lerp(Rotator) (.rotation (Variables|Default|GetStartLeft)) (Math|Rotator|MakeRotator (.roll (.rotation _startleft)) (.pitch (.rotation _startleft)) 1.2e+02) _alpha true) false false)))))

(event EventBeginPlay
  (Variables|Default|SetStartLeft (Transformation|GetRelativeTransform (Variables|Default|GetLeft)))
  (Variables|Default|SetStartRighrt (Transformation|GetRelativeTransform (Variables|Default|GetRight))))

(fn ConstructionScript)

(fn Interact
  (params (HasIntracted? :type Boolean) (Player :type BP%20Base%20Souls%20Chap%20Object%20Reference))
  (return 0 false))