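; BP_SmallDoor is a one-way interactable door that swings open once and stays open.
; Box overlaps show or clear an interaction popup on actors implementing BPI_Player.
; The interact event sets the Open flag, plays a sound and runs a timeline that rotates the whole actor from the mesh's initial relative rotation toward a fixed 180-degree yaw.
; The separate Interact function only returns failure.
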(event OnComponentBeginOverlap(Box)
  (params (OverlappedComponent :type Primitive%20Component%20Object%20Reference) (OtherActor :type Actor%20Object%20Reference) (OtherComp :type Primitive%20Component%20Object%20Reference) (OtherBodyIndex :type Integer) (bFromSweep :type Boolean) (SweepResult :type Hit%20Result%20Structure%20%28by%20ref%29))
  (if (and (Utilities|DoesObjectImplementInterface OtherActor "/Game/SoulsLlike/Light/BluePrints/Interfaces/BPI_Player.BPI_Player_C") (not (Variables|Default|GetOpen?)))
    (Class|BPIPlayer|Popup(Message) OtherActor (Variables|Default|GetIntract%20With) 0 "NewEnumerator0")
    (else
      (Class|BPIPlayer|LeavePopUp(Message) OtherActor))))

(event OnComponentEndOverlap(Box)
  (params (OverlappedComponent :type Primitive%20Component%20Object%20Reference) (OtherActor :type Actor%20Object%20Reference) (OtherComp :type Primitive%20Component%20Object%20Reference) (OtherBodyIndex :type Integer))
  (if (Utilities|DoesObjectImplementInterface OtherActor "/Game/SoulsLlike/Light/BluePrints/Interfaces/BPI_Player.BPI_Player_C")
    (Class|BPIPlayer|LeavePopUp(Message) OtherActor)))

(event Custom|Intract_1_1
  (params (HasIntracted? :type Boolean))
  (if (and HasIntracted? (not (Variables|Default|GetOpen?)))
    (Variables|Default|SetOpen? true)
    (Audio|PlaySoundatLocation "/Game/SoulsLlike/Light/Sound/Effects/SW_Dungeon_Door_Open_Wet_B.SW_Dungeon_Door_Open_Wet_B" (Transformation|GetSocketLocation (Variables|Debug|GetStaticMeshComponent) "None") "0, 0, 0" 1.0 1.0 0.0 0 0 0 0)
    (bind _alpha (Timeline|Timeline Play)
      (:Update
        (Transformation|SetActorRotation (Math|Rotator|Lerp(Rotator) (.rotation (Variables|Default|GetSart)) (Math|Rotator|MakeRotator 0.0 0.0 1.8e+02) _alpha true))))))

(event EventBeginPlay
  (Variables|Default|SetSart (Transformation|GetRelativeTransform (Variables|Debug|GetStaticMeshComponent))))

(fn ConstructionScript)

(fn Interact
  (params (HasIntracted? :type Boolean) (Player :type BP%20Base%20Souls%20Chap%20Object%20Reference))
  (return 0 false))